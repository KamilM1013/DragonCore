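; Construction-script foliage spawner that fills the area enclosed by a spline with instanced meshes.
; It creates or clears a HISM per ProceduralElements entry, then steps a grid across the spline's bounds, keeping points that pass a ray-crossing polygon test.
; Downward line traces at those points place every element, with randomized offset, rotation and scale computed through WS and LS helper components.
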(fn `DoIntersect`
  (params (P1 :type "Vector Structure") (Q1 :type "Vector Structure") (P2 :type "Vector Structure") (Q2 :type "Vector Structure"))
  (returns (Intersect :type Boolean))
  (locals (O1 :type Integer :default 0) (O2 :type Integer :default 0) (O3 :type Integer :default 0) (O4 :type Integer :default 0))
  (bind _orientation (`self.Orientation` P1 Q1 P2))
  (bind _output_get (set `local.O1` _orientation))
  (bind _orientation_2 (`self.Orientation` P1 Q1 Q2))
  (bind _output_get_2 (set `local.O2` _orientation_2))
  (bind _orientation_3 (`self.Orientation` P2 Q2 P1))
  (bind _output_get_3 (set `local.O3` _orientation_3))
  (bind _orientation_4 (`self.Orientation` P2 Q2 Q1))
  (bind _output_get_4 (set `local.O4` _orientation_4))
  (return (and (!= _output_get _output_get_2) (!= _output_get_3 _output_get_4))))

(fn `Get Min Max`
  (returns (pMin1 :type "Vector Structure") (pMax1 :type "Vector Structure"))
  (locals (Distance :type "Float (double-precision)") (pMin :type "Vector Structure") (pMax :type "Vector Structure"))
  (bind (_pmin_x _pmin_y _pmin_z) (`KismetMathLibrary.BreakVector` (`local.pMin`)))
  (bind (_pmax_x _pmax_y _pmax_z) (`KismetMathLibrary.BreakVector` (`local.pMax`)))
  (bind _returnvalue (`SplineComponent.GetLocationAtDistanceAlongSpline` (`self.Spline`) (`local.Distance`) "World"))
  (set `local.pMin` _returnvalue)
  (set `local.pMax` _returnvalue)
  (while (< (`local.Distance`) (`SplineComponent.GetSplineLength` (`self.Spline`)))
    (set `local.pMin` (`KismetMathLibrary.MakeVector` (`KismetMathLibrary.FMin` (.x _returnvalue) _pmin_x) (`KismetMathLibrary.FMin` (.y _returnvalue) _pmin_y) (`KismetMathLibrary.FMin` (.z _returnvalue) _pmin_z)))
    (set `local.pMax` (`KismetMathLibrary.MakeVector` (`KismetMathLibrary.FMax` (.x _returnvalue) _pmax_x) (`KismetMathLibrary.FMax` (.y _returnvalue) _pmax_y) (`KismetMathLibrary.FMax` (.z _returnvalue) _pmax_z)))
    (set `local.Distance` (+ (`local.Distance`) 100.0)))
  (return (`local.pMin`) (`local.pMax`)))

(fn `IsInsidePolygon`
  (params (P :type "Vector Structure"))
  (returns (`IsInside?` :type Boolean))
  (locals (IntersectionCount :type Integer))
  (bind _spline (`self.Spline`))
  (bind _returnvalue (`SplineComponent.GetNumberOfSplinePoints` _spline))
  (for _index (range _returnvalue)
    (bind _intersect (`self.DoIntersect` P (+ (`self.pMinG`) (-100.0 0.0 0.0)) (`SplineComponent.GetLocationAtSplinePoint` _spline _index "World") (`SplineComponent.GetLocationAtSplinePoint` _spline (mod (+ _index 1) _returnvalue) "World")))
    (if _intersect
      (`/Engine/EditorBlueprintResources/StandardMacros.IncrementInt` (`local.IntersectionCount`))))
  (return (!= (mod (`local.IntersectionCount`) 2) 0)))

(fn `Orientation`
  (params (P :type "Vector Structure") (Q :type "Vector Structure") (R :type "Vector Structure"))
  (returns (orientation :type Integer))
  (bind _x (.x Q))
  (bind _y (.y Q))
  (bind _returnvalue (- (* (- _y (.y P)) (- (.x R) _x)) (* (- _x (.x P)) (- (.y R) _y))))
  (if (== _returnvalue 0.0)
    (return 0)
    (elif (> _returnvalue 0.0)
      (return 1)
      (else
        (return 2)))))

(fn `UserConstructionScript`
  (locals (pMin :type "Vector Structure" :default (0.0 0.0 0.0)) (pMax :type "Vector Structure" :default (0.0 0.0 0.0)) (tempX :type "Float (double-precision)") (tempY :type "Float (double-precision)"))
  (bind _proceduralelements (`self.ProceduralElements`))
  (bind _hism_current (`self.HISM current`))
  (bind _ls (`self.LS`))
  (bind (_pmaxg_x _pmaxg_y _pmaxg_z) (`KismetMathLibrary.BreakVector` (`self.pMaxG`)))
  (bind (_pmaxg_x_2 _pmaxg_y_2) (`KismetMathLibrary.BreakVector` (`self.pMaxG`)))
  (bind _volumeheight (`self.VolumeHeight`))
  (bind (_pming_x _pming_y) (`KismetMathLibrary.BreakVector` (`self.pMinG`)))
  (bind _pmaxg_x_3 (`KismetMathLibrary.BreakVector` (`self.pMaxG`)))
  (bind _pming_x_2 (`KismetMathLibrary.BreakVector` (`self.pMinG`)))
  (for (_array_element _array_index) _proceduralelements
    (`/Engine/EditorBlueprintResources/StandardMacros.IsValid` (`.HISM_42_BC8631CD48A82FA7A1996A9D4D52ED73` (break `/Game/StylizedProvencal/Blueprints/ProceduralElements` _array_element))
      (:`Is Valid`
        _)
      (:`Is Not Valid`
        (bind _returnvalue (`AddComponent|NODE_AddHierarchicalInstancedStaticMeshComponent-0`))
        (bind _output_get (set `self.HISM current` _returnvalue))
        (setmembers `/Game/StylizedProvencal/Blueprints/ProceduralElements` :`StructRef` (`|GetArrayItem` _proceduralelements _array_index) :`HISM` _output_get)))
    (`StaticMeshComponent.SetStaticMesh` _hism_current (break `/Game/StylizedProvencal/Blueprints/ProceduralElements` _array_element))
    (`InstancedStaticMeshComponent.ClearInstances` _hism_current))
  (bind (_pmin1 _pmax1) (`self.Get Min Max`))
  (set `self.pMinG` _pmin1)
  (set `self.pMaxG` _pmax1)
  (`KismetSystemLibrary.LineTraceSingle` :`Start` _pmin1 :`End` _pmax1 :`TraceChannel` "TraceTypeQuery1" :`DrawTime` 2.0)
  (set `local.tempY` _pming_y)
  (while (<= (`local.tempY`) _pmaxg_y_2)
    (set `local.tempX` _pming_x_2)
    (while (< (`local.tempX`) _pmaxg_x_3)
      (bind _output_get_2 (set `self.Ptemp` (`KismetMathLibrary.MakeVector` (`local.tempX`) (`local.tempY`) _pmaxg_z)))
      (bind _isinside_ (`self.IsInsidePolygon` _output_get_2))
      (if _isinside_
        (bind (_outhit _returnvalue_2) (`KismetSystemLibrary.LineTraceSingle` :`Start` (+ _output_get_2 (`KismetMathLibrary.MakeVector` 0.0 0.0 _volumeheight)) :`End` (- _output_get_2 (`KismetMathLibrary.MakeVector` 0.0 0.0 _volumeheight)) :`TraceChannel` "TraceTypeQuery1" :`DrawTime` 3.0))
        (if _returnvalue_2
          (for _array_element_2 (`self.ProceduralElements`)
            (`SceneComponent.K2_SetWorldLocationAndRotation` (`self.WS`) (`.Location` (`GameplayStatics.BreakHitResult` _outhit)) (struct) false false)
            (bind (_mesh _distance _scalemax _scalemin _offset _offsetvariation _rotation _rotationvariation _keepvertical _verticalcheckdistance _hism) (break `/Game/StylizedProvencal/Blueprints/ProceduralElements` _array_element_2))
            (`SceneComponent.K2_SetRelativeLocationAndRotation` _ls (+ _offset (`KismetMathLibrary.MakeVector` (* (.x _offsetvariation) (`KismetMathLibrary.RandomFloatInRange` -1.0 1.0)) (* (.y _offsetvariation) (`KismetMathLibrary.RandomFloatInRange` -1.0 1.0)) (* (.z _offsetvariation) (`KismetMathLibrary.RandomFloatInRange` -1.0 1.0)))) _rotation false false)
            (`SceneComponent.K2_AddRelativeRotation` _ls (`KismetMathLibrary.MakeRotator` (`KismetMathLibrary.RandomFloatInRange` 0.0 (.roll _rotationvariation)) (`KismetMathLibrary.RandomFloatInRange` 0.0 (.pitch _rotationvariation)) (`KismetMathLibrary.RandomFloatInRange` 0.0 (.yaw _rotationvariation))) false false)
            (`SceneComponent.SetWorldScale3D` (`self.LS`) (* (1.0 1.0 1.0) (`KismetMathLibrary.RandomFloatInRange` _scalemin _scalemax)))
            (`InstancedStaticMeshComponent.AddInstance` _hism (`SceneComponent.K2_GetComponentToWorld` (`self.LS`)) true))))
      (set `local.tempX` (+ (`local.tempX`) (`self.DistanceX`))))
    (set `local.tempY` (+ (`local.tempY`) (`self.DistanceY`)))))