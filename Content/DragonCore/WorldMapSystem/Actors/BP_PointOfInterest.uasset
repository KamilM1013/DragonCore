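; BP_PointOfInterest is a world map point of interest that starts undiscovered and is revealed when the player comes within range.
; Shortly after BeginPlay it creates a compass marker with the undiscovered material.
; Overlapping the construction-sized discovery sphere switches the marker to its type material and notifies the overlapping actor's BPC_WorldMap once.
; OnDiscovered destroys the sphere, while GetMapIconData supplies location and question-mark icon data for the map.
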(event `self.ReceiveBeginPlay`
  (bind _marker (`self.Marker`))
  (`KismetSystemLibrary.Delay` 0.2)
  (bind _returnvalue (`|CreateWidget` "/Game/DragonCore/UI_HUD/WDG_CompassMarker.WDG_CompassMarker_C"))
  (set `self.Marker` _returnvalue)
  (`UserWidget.AddToViewport` _marker 0)
  (`/Game/DragonCore/UI_HUD/WDG_CompassMarker.InitMarker` _marker (`self.Marker Color`) (`self.Undiscovered`) self))

(event `self.DiscoverRange.OnComponentBeginOverlap`
  (params (OverlappedComponent :type "PrimitiveComponent Object Reference") (OtherActor :type "Actor Object Reference") (OtherComp :type "PrimitiveComponent Object Reference") (OtherBodyIndex :type Integer) (bFromSweep :type Boolean) (SweepResult :type "HitResult Structure (by ref)"))
  (bind _returnvalue (`self.GetComponentByClass` OtherActor "/Game/DragonCore/WorldMapSystem/Actors/BPC_WorldMap.BPC_WorldMap_C"))
  (bind _marker (`self.Marker`))
  (`|ExecutionSequence`
    (:`then_0`
      (cast `/Game/ThirdPerson/Blueprints/BP_ThirdPersonCharacter` OtherActor)
      (`Widget.RemoveFromParent` (`self.Marker`))
      (`UserWidget.AddToViewport` _marker 0)
      (`/Game/DragonCore/UI_HUD/WDG_CompassMarker.InitMarker` _marker (`self.Marker Color`) (`self.TypeOfPOI_Compass`) self))
    (:`then_1`
      (`/Engine/EditorBlueprintResources/StandardMacros.IsValid` _returnvalue
        (:`Is Valid`
          (`/Engine/EditorBlueprintResources/StandardMacros.DoOnce` false
            (:`Completed`
              (`/Game/DragonCore/WorldMapSystem/Actors/BPC_WorldMap.OnDiscoveredPointOfInterest` _returnvalue self (`self.TypeOfPOI_Map`)))))))))

(event `OnDiscovered`
  (`ActorComponent.K2_DestroyComponent` (`self.DiscoverRange`)))

(fn `GetMapIconData`
  (returns (Location :type "Vector Structure") (Icon :type "Texture2D Object Reference") (IconSize :type "Vector2D Structure") (`Rotation Yaw` :type "Float (double-precision)") (`World Actor` :type "Actor Object Reference"))
  (return (`self.K2_GetActorLocation`) "/Game/DragonCore/WorldMapSystem/Textures/MapIconQuestionMark.MapIconQuestionMark" (30.0 30.0) 0.0 self))

(fn `UserConstructionScript`
  (`SphereComponent.SetSphereRadius` (`self.DiscoverRange`) (`self.DiscoverRadius`) false))