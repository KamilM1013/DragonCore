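; Flight component that lets the player character take off, fly along the camera direction with vertical input, and land automatically.
; Takeoff is gated by combat action and target-lock flags, then a montage switches movement to Flying, zooms the camera and disables combat actions.
; While flying, Tick feeds a delayed timer that line-traces below the mesh.
; A hit at low speed plays the landing montage and restores walking, camera and combat, guarded by a resettable DoOnce.
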(event `Init Flight`
  (params (PlayerCharacter :type "/Game/ThirdPerson/Blueprints/BP_ThirdPersonCharacter Object Reference"))
  ;[0.05127 0.05127 0.05127] Setup player character references
  (bind _output_get (set `self.PlayerCharacter` PlayerCharacter))
  (set `self.Mesh` (`Character.Mesh` _output_get))
  (set `self.Follow Camera` (`/Game/ThirdPerson/Blueprints/BP_ThirdPersonCharacter.FollowCamera` _output_get))
  (set `self.Character Movement` (`Character.CharacterMovement` _output_get)))

(event `EnhancedInput|/Game/ThirdPerson/Input/Actions/IA_UpDown`
  (params (ActionValue :type "Vector2D Structure") (ElapsedSeconds :type "Float (double-precision)") (TriggeredSeconds :type "Float (double-precision)") (InputAction :type "InputAction Object Reference" :default "/Game/ThirdPerson/Input/Actions/IA_UpDown.IA_UpDown"))
  ;[0.05127 0.05127 0.05127] Move Up/Down
  (:`Triggered`
    (bind _output_get (set `self.MoveUp` ActionValue_Y))
    (`Pawn.AddMovementInput` (`self.PlayerCharacter`) (0.0 0.0 1.0) _output_get false)))

(event `EnhancedInput|/Game/ThirdPerson/Input/Actions/IA_Move`
  (params (ActionValue :type "Vector2D Structure") (ElapsedSeconds :type "Float (double-precision)") (TriggeredSeconds :type "Float (double-precision)") (InputAction :type "InputAction Object Reference" :default "/Game/ThirdPerson/Input/Actions/IA_Move.IA_Move"))
  ;[0.05127 0.05127 0.05127] Add movement force for flight
  (:`Triggered`
    (if (`self.isFlying`)
      (`Pawn.AddMovementInput` (`self.PlayerCharacter`) (`SceneComponent.GetForwardVector` (`self.Follow Camera`)) ActionValue_Y false))))

(event `FlightModeTriggered`
  (bind (_candoaction _nottargetlocked) (`self.CheckForFlags`))
  ;[0.05127 0.05127 0.05127] Switch to Flying Mode
  (if (and _candoaction _nottargetlocked)
    (`self.Start Flying`)))

(event `Start Flying`
  (bind _playercharacter (`self.PlayerCharacter`))
  (bind _character_movement (`self.Character Movement`))
  ;[0.05127 0.05127 0.05127] Start Flying
  (if (not (`self.isFlying`))
    (`self.CanPlayAnimation`
      (:`Play Animation`
        (set `Pawn.bUseControllerRotationYaw` true _playercharacter)
        (set `/Game/DragonCore/Combat/BPC_CombatSystem.canDoAction` false (`self.Get CombatSystem Ref`))
        (`|PlayMontage` (`self.Mesh`) "/Game/DragonCore/PlayerCharacters/Noxturn/Animations/Montages/Flight/JumpTransitionNox.JumpTransitionNox"
          (:`OnInterrupted`
            _)
          (:`OnNotifyBegin`
            _))
        (set `Pawn.bUseControllerRotationYaw` false _playercharacter)
        (set `self.isFlying` true)
        (`CharacterMovementComponent.SetMovementMode` _character_movement "MOVE_Flying" 0)
        (set `/Game/DragonCore/Combat/BPC_CombatSystem.canDoAction` false (`self.Get CombatSystem Ref`))
        (set `CharacterMovementComponent.bUseControllerDesiredRotation` true _character_movement)
        (set `CharacterMovementComponent.bOrientRotationToMovement` false _character_movement)
        (`/Game/ThirdPerson/Blueprints/BP_ThirdPersonCharacter.ZoomIn` (`self.PlayerCharacter`))
        (`self.ResetStopFlying`)))))

(event `self.ReceiveTick`
  (params (DeltaSeconds :type "Float (single-precision)"))
  ;[0.05127 0.05127 0.05127] Check if can land
  (if (`self.isFlying`)
    (`self.Land` -125.0)))

(event `Land`
  (params (`Z Height Needed To Land` :type "Float (single-precision)"))
  ;[0.05127 0.05127 0.05127] Carry out land procedure
  (if (`self.isFlying`)
    (`KismetSystemLibrary.Delay` 2.0)
    (bind _returnvalue (`KismetSystemLibrary.K2_SetTimerDelegate` (delegate `Land Tick`) 0.3))
    (set `self.Land Timer` _returnvalue)
    (else
      (`KismetSystemLibrary.K2_ClearAndInvalidateTimerHandle` (`self.Land Timer`)))))

(event `Land Tick`
  ;[0.05127 0.05127 0.05127] Carry out land procedure
  (bind _success (`self.Land Line Trace` (stale `Land` `Z Height Needed To Land`)))
  (if (and _success (< (`KismetMathLibrary.VSize` (`MovementComponent.Velocity` (`self.Character Movement`))) 600.0))
    (`self.Stop Flying`)
    (`KismetSystemLibrary.K2_ClearAndInvalidateTimerHandle` (`self.Land Timer`))))

(event `Stop Flying`
  (bind _playercharacter (`self.PlayerCharacter`))
  (bind _character_movement (`self.Character Movement`))
  ;[0.05127 0.05127 0.05127] Stop Flying
  (`/Engine/EditorBlueprintResources/StandardMacros.DoOnce` false :!label _label
    (:`Completed`
      (`self.CanPlayAnimation`
        (:`Play Animation`
          (set `Pawn.bUseControllerRotationYaw` false _playercharacter)
          (`|PlayMontage` (`self.Mesh`) "/Game/DragonCore/PlayerCharacters/Noxturn/Animations/Montages/Flight/LandTransitionNox.LandTransitionNox"
            (:`OnBlendOut`
              (set `Pawn.bUseControllerRotationYaw` false _playercharacter))
            (:`OnInterrupted`
              _)
            (:`OnNotifyBegin`
              _))
          (`CharacterMovementComponent.SetMovementMode` _character_movement "MOVE_Walking" 0)
          (set `self.isFlying` false)
          (set `/Game/DragonCore/Combat/BPC_CombatSystem.canDoAction` true (`self.Get CombatSystem Ref`))
          (set `CharacterMovementComponent.bUseControllerDesiredRotation` false _character_movement)
          (set `CharacterMovementComponent.bOrientRotationToMovement` true _character_movement)
          (`/Game/ThirdPerson/Blueprints/BP_ThirdPersonCharacter.ZoomOut` (`self.PlayerCharacter`)))))))

(event `ResetStopFlying`
  ;[0.05127 0.05127 0.05127] Stop Flying
  (goto _label :!via `Reset`))

(fn `Land Line Trace`
  (params (`Z Height Needed To Land` :type "Float (single-precision)"))
  (returns (Success :type Boolean))
  (bind _mesh (`self.Mesh`))
  (bind _returnvalue (`SceneComponent.K2_GetComponentLocation` _mesh))
  (if (`self.isFlying`)
    (bind (_outhit _returnvalue_2) (`KismetSystemLibrary.LineTraceSingle` _returnvalue (+ _returnvalue (* (`SceneComponent.GetUpVector` _mesh) (`local.Z Height Needed To Land`))) "TraceTypeQuery1"))
    (return _returnvalue_2)))