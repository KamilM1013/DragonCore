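; Stats component for the player, dummy, master enemy and deprecated AI, tracking health, rage, XP and level.
; BeginPlay casts the owner to set type flags and fill its bars; stat functions then update values and widgets directly.
; Tick lerps a back health bar toward current health for a trailing damage effect.
; XP overflow loops into level-ups that scale stats, play sounds and notify the player; mana functions are disconnected stubs.
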(event `self.ReceiveBeginPlay`
  ;[0.05127 0.05127 0.05127] Initializing all Progress Bars
  (`KismetSystemLibrary.DelayUntilNextTick`)
  (bind _asbp_third_person_character (cast `/Game/ThirdPerson/Blueprints/BP_ThirdPersonCharacter` (`self.GetOwner`))
    (:`then`
      (set `self.Player Character` _asbp_third_person_character)
      (set `self.isPlayer?` true)
      (set `self.isMasterEnemy?` false)
      (set `self.isDeprecatedAI?` false)
      (`ProgressBar.SetPercent` (`/Game/DragonCore/HUD/Widgets/WB_HUD.RageBar` (`/Game/ThirdPerson/Blueprints/BP_ThirdPersonCharacter.HUD_Widget` (`self.Player Character`))) (`KismetMathLibrary.MapRangeClamped` (`self.Current Rage`) 0.0 (`self.Max Rage`) 0.0 1.0))
      (`ProgressBar.SetPercent` (`/Game/DragonCore/HUD/Widgets/WB_Level.XPBar` (`/Game/ThirdPerson/Blueprints/BP_ThirdPersonCharacter.HUD Level` (`self.Player Character`))) (`KismetMathLibrary.MapRangeClamped` (`self.XP`) 0.0 (`self.Max XP`) 0.0 1.0))
      (`TextBlock.SetText` (`/Game/DragonCore/HUD/Widgets/WB_Level.Level` (`/Game/ThirdPerson/Blueprints/BP_ThirdPersonCharacter.HUD Level` (`self.Player Character`))) (`KismetTextLibrary.Conv_IntToText` (`self.Level`))))
    (:`CastFailed`
      (bind _asbp_dummy (cast `/Game/DragonCore/AI_Classes/BP_Dummy` (`self.GetOwner`))
        (:`then`
          (set `self.Dummy` _asbp_dummy)
          (set `self.isPlayer?` false)
          (set `self.isMasterEnemy?` false)
          (set `self.isDeprecatedAI?` false))
        (:`CastFailed`
          (bind _asmaster_enemy (cast `/Game/DragonCore/AI_Classes/Master_Enemy/Master_Enemy` (`self.GetOwner`))
            (:`then`
              (set `self.MasterEnemy` _asmaster_enemy)
              (set `self.isPlayer?` false)
              (set `self.isMasterEnemy?` true)
              (set `self.isDeprecatedAI?` false))
            (:`CastFailed`
              (bind _asbp_deprecated_ai (cast `/Game/DragonCore/AI_Classes/DeprecatedAI/BP_DeprecatedAI` (`self.GetOwner`)))
              (set `self.DeprecatedAI` _asbp_deprecated_ai)
              (set `self.isPlayer?` false)
              (set `self.isMasterEnemy?` false)
              (set `self.isDeprecatedAI?` true)))))))
  (`ProgressBar.SetPercent` (select `bool` (`self.isDeprecatedAI?`) :`false` (select `bool` (`self.isMasterEnemy?`) :`false` (select `bool` (`self.isPlayer?`) :`false` (`/Game/DragonCore/HUD/Widgets/WB_DummyHealthBar.HealthBar` (`/Game/DragonCore/AI_Classes/BP_Dummy.Health Bar UI` (`self.Dummy`))) :`true` (`/Game/DragonCore/HUD/Widgets/WB_HUD.HealthBar` (`/Game/ThirdPerson/Blueprints/BP_ThirdPersonCharacter.HUD_Widget` (`self.Player Character`)))) :`true` (`/Game/DragonCore/HUD/Widgets/WB_DummyHealthBar.HealthBar` (`/Game/DragonCore/AI_Classes/Master_Enemy/Master_Enemy.Health Bar UI` (`self.MasterEnemy`)))) :`true` (`/Game/DragonCore/HUD/Widgets/WB_DummyHealthBar.HealthBar` (`/Game/DragonCore/AI_Classes/DeprecatedAI/BP_DeprecatedAI.Health Bar UI` (`self.DeprecatedAI`)))) (`KismetMathLibrary.MapRangeClamped` (`self.Current Health`) 0.0 (`self.Max Health`) 0.0 1.0)))

(event `self.ReceiveTick`
  (params (DeltaSeconds :type "Float (single-precision)"))
  ;[0.05127 0.05127 0.05127] Adds effect to Health Bar while decreasing health
  (bind _asmaster_enemy (cast `/Game/DragonCore/AI_Classes/Master_Enemy/Master_Enemy` (`self.GetOwner`))
    (:`then`
      (bind _healthbarback (`/Game/DragonCore/HUD/Widgets/WB_DummyHealthBar.HealthBarBack` (`/Game/DragonCore/AI_Classes/Master_Enemy/Master_Enemy.Health Bar UI` _asmaster_enemy)))
      (`ProgressBar.SetPercent` _healthbarback (`KismetMathLibrary.Lerp` (`ProgressBar.Percent` _healthbarback) (/ (`self.Current Health`) (`self.Max Health`)) 0.05)))
    (:`CastFailed`
      (bind _asbp_dummy (cast `/Game/DragonCore/AI_Classes/BP_Dummy` (`self.GetOwner`))
        (:`then`
          (bind _healthbarback_2 (`/Game/DragonCore/HUD/Widgets/WB_DummyHealthBar.HealthBarBack` (`/Game/DragonCore/AI_Classes/BP_Dummy.Health Bar UI` _asbp_dummy)))
          (`ProgressBar.SetPercent` _healthbarback_2 (`KismetMathLibrary.Lerp` (`ProgressBar.Percent` _healthbarback_2) (/ (`self.Current Health`) (`self.Max Health`)) 0.05)))
        (:`CastFailed`
          (bind _asbp_third_person_character (cast `/Game/ThirdPerson/Blueprints/BP_ThirdPersonCharacter` (`self.GetOwner`))
            (:`then`
              (bind _healthbarback_3 (`/Game/DragonCore/HUD/Widgets/WB_HUD.HealthBarBack` (`/Game/ThirdPerson/Blueprints/BP_ThirdPersonCharacter.HUD_Widget` _asbp_third_person_character)))
              (`ProgressBar.SetPercent` _healthbarback_3 (`KismetMathLibrary.Lerp` (`ProgressBar.Percent` _healthbarback_3) (/ (`self.Current Health`) (`self.Max Health`)) 0.05)))
            (:`CastFailed`
              (bind _asbp_deprecated_ai (cast `/Game/DragonCore/AI_Classes/DeprecatedAI/BP_DeprecatedAI` (`self.GetOwner`)))
              (bind _healthbarback_4 (`/Game/DragonCore/HUD/Widgets/WB_DummyHealthBar.HealthBarBack` (`/Game/DragonCore/AI_Classes/DeprecatedAI/BP_DeprecatedAI.Health Bar UI` _asbp_deprecated_ai)))
              (`ProgressBar.SetPercent` _healthbarback_4 (`KismetMathLibrary.Lerp` (`ProgressBar.Percent` _healthbarback_4) (/ (`self.Current Health`) (`self.Max Health`)) 0.05)))))))))

(fn `Decrease Health`
  (params (Damage :type "Float (double-precision)"))
  (returns (`isPlayerDead?` :type Boolean))
  (if (not (<= (`self.Current Health`) 0.0))
    (bind _output_get (set `self.Current Health` (- (`self.Current Health`) Damage)))
    (`ProgressBar.SetPercent` (select `bool` (`self.isMasterEnemy?`) :`false` (select `bool` (`self.isPlayer?`) :`false` (`/Game/DragonCore/HUD/Widgets/WB_DummyHealthBar.HealthBar` (`/Game/DragonCore/AI_Classes/BP_Dummy.Health Bar UI` (`self.Dummy`))) :`true` (`/Game/DragonCore/HUD/Widgets/WB_HUD.HealthBar` (`/Game/ThirdPerson/Blueprints/BP_ThirdPersonCharacter.HUD_Widget` (`self.Player Character`)))) :`true` (`/Game/DragonCore/HUD/Widgets/WB_DummyHealthBar.HealthBar` (`/Game/DragonCore/AI_Classes/Master_Enemy/Master_Enemy.Health Bar UI` (`self.MasterEnemy`)))) (`KismetMathLibrary.MapRangeClamped` _output_get 0.0 (`self.Max Health`) 0.0 1.0))
    (if (<= (`self.Current Health`) 0.0)
      _
      (else
        (return false))))
  (return true))

(fn `Decrease Mana`
  (params (`Mana Depleted` :type "Float (double-precision)"))
  (returns (`No Mana` :type Boolean)))

(fn `Decrease Rage`
  (params (`Rage Depleted` :type "Float (double-precision)"))
  (returns (`No Rage` :type Boolean))
  (if (not (<= (`self.Current Rage`) 0.0))
    (bind _output_get (set `self.Current Rage` (- (`self.Current Rage`) `Rage Depleted`)))
    (`ProgressBar.SetPercent` (`/Game/DragonCore/HUD/Widgets/WB_HUD.RageBar` (`/Game/ThirdPerson/Blueprints/BP_ThirdPersonCharacter.HUD_Widget` (`self.Player Character`))) (`KismetMathLibrary.MapRangeClamped` _output_get 0.0 (`self.Max Rage`) 0.0 1.0))
    (if (<= (`self.Current Rage`) 0.0)
      _
      (else
        (return false))))
  (return true))

(fn `Increase Health`
  (params (`Added Health` :type "Float (double-precision)"))
  (bind _max_health (`self.Max Health`))
  (bind _healthbar (`/Game/DragonCore/HUD/Widgets/WB_HUD.HealthBar` (`/Game/ThirdPerson/Blueprints/BP_ThirdPersonCharacter.HUD_Widget` (`self.Player Character`))))
  (bind _output_get (set `self.Current Health` (+ (`self.Current Health`) `Added Health`)))
  (if (> _output_get (`self.Max Health`))
    (bind _output_get_2 (set `self.Current Health` _max_health))
    (`ProgressBar.SetPercent` _healthbar (`KismetMathLibrary.MapRangeClamped` _output_get_2 0.0 _max_health 0.0 1.0))
    (else
      (`ProgressBar.SetPercent` _healthbar (`KismetMathLibrary.MapRangeClamped` _output_get 0.0 _max_health 0.0 1.0)))))

(fn `Increase Level`
  (params (`Added Level` :type Integer))
  (set `self.Level` (+ (`self.Level`) `Added Level`))
  (set `self.XP` (- (`self.XP`) (`self.Max XP`)))
  (set `self.Max XP` (`KismetMathLibrary.Conv_IntToDouble` (`KismetMathLibrary.FFloor` (* (`self.Max XP`) 1.5))))
  (set `self.Magic Damage` (`KismetMathLibrary.Conv_IntToDouble` (`KismetMathLibrary.FFloor` (* (`self.Magic Damage`) 1.2))))
  (set `self.Max Health` (`KismetMathLibrary.Conv_IntToDouble` (`KismetMathLibrary.FFloor` (* (`self.Max Health`) 1.2))))
  (set `self.Damage` (`KismetMathLibrary.Conv_IntToDouble` (`KismetMathLibrary.FFloor` (* (`self.Damage`) 1.2))))
  (`TextBlock.SetText` (`/Game/DragonCore/HUD/Widgets/WB_Level.Level` (`/Game/ThirdPerson/Blueprints/BP_ThirdPersonCharacter.HUD Level` (`self.Player Character`))) (`KismetTextLibrary.Conv_IntToText` (`self.Level`)))
  (`GameplayStatics.PlaySound2D` "/Game/DragonCore/Audio/UI/LevelUp.LevelUp" 1.0 1.0 0.0 null null)
  (`GameplayStatics.PlaySound2D` "/Game/DragonCore/Audio/UI/LevelUp2.LevelUp2" 1.0 1.0 0.0 null null)
  (`/Game/ThirdPerson/Blueprints/BP_ThirdPersonCharacter.LevelUp` (`self.Player Character`)))

(fn `Increase Mana`
  (params (`Added Mana` :type "Float (double-precision)")))

(fn `Increase Max Health`
  (params (`Added Health` :type "Float (double-precision)"))
  (bind _output_get (set `self.Max Health` (+ (`self.Max Health`) `Added Health`)))
  (`ProgressBar.SetPercent` (select `bool` (`self.isPlayer?`) :`false` (`/Game/DragonCore/HUD/Widgets/WB_DummyHealthBar.HealthBar` (`/Game/DragonCore/AI_Classes/Master_Enemy/Master_Enemy.Health Bar UI` (`self.MasterEnemy`))) :`true` (`/Game/DragonCore/HUD/Widgets/WB_HUD.HealthBar` (`/Game/ThirdPerson/Blueprints/BP_ThirdPersonCharacter.HUD_Widget` (`self.Player Character`)))) (`KismetMathLibrary.FClamp` _output_get)))

(fn `Increase Max Mana`
  (params (`Added Mana` :type "Float (double-precision)")))

(fn `Increase Rage`
  (params (`Added Rage` :type "Float (double-precision)"))
  (bind _max_rage (`self.Max Rage`))
  (bind _ragebar (`/Game/DragonCore/HUD/Widgets/WB_HUD.RageBar` (`/Game/ThirdPerson/Blueprints/BP_ThirdPersonCharacter.HUD_Widget` (`self.Player Character`))))
  (bind _output_get (set `self.Current Rage` (+ (`self.Current Rage`) `Added Rage`)))
  (if (> _output_get (`self.Max Rage`))
    (bind _output_get_2 (set `self.Current Rage` _max_rage))
    (`ProgressBar.SetPercent` _ragebar (`KismetMathLibrary.MapRangeClamped` _output_get_2 0.0 _max_rage 0.0 1.0))
    (else
      (`ProgressBar.SetPercent` _ragebar (`KismetMathLibrary.MapRangeClamped` _output_get 0.0 _max_rage 0.0 1.0)))))

(fn `Increase XP`
  (params (`Added XP` :type "Float (double-precision)"))
  (bind _output_get (set `self.XP` (+ (`self.XP`) `Added XP`)))
  (while (>= _output_get (`self.Max XP`))
    (`self.Increase Level` 1)
    (`ProgressBar.SetPercent` (`/Game/DragonCore/HUD/Widgets/WB_Level.XPBar` (`/Game/ThirdPerson/Blueprints/BP_ThirdPersonCharacter.HUD Level` (`self.Player Character`))) (`KismetMathLibrary.MapRangeClamped` (`self.XP`) 0.0 (`self.Max XP`) 0.0 1.0) :!label _label))
  (goto _label))