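; BP_Marker is a placeable marker actor that shows itself through a WDG_CompassMarker widget in its MarkerColor.
; Shortly after BeginPlay it creates the widget, adds it to the viewport and initializes it with the standard marker material and itself as owner.
; Any overlap on the Trigger component re-adds that widget and re-initializes it with the exclamation marker material.
; The construction script tints the static mesh with the same color.
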(event `self.ReceiveBeginPlay`
  (bind _marker (`self.Marker`))
  (`KismetSystemLibrary.Delay` 0.2)
  (bind _returnvalue (`|CreateWidget` "/Game/DragonCore/UI/WDG_CompassMarker.WDG_CompassMarker_C"))
  (set `self.Marker` _returnvalue)
  (`UserWidget.AddToViewport` _marker 0)
  (`/Game/DragonCore/UI/WDG_CompassMarker.InitMarker` _marker (`self.Marker Color`) "/Game/DragonCore/UI/MInst_Marker.MInst_Marker" self))

(event `self.Trigger.OnComponentBeginOverlap`
  (params (OverlappedComponent :type "PrimitiveComponent Object Reference") (OtherActor :type "Actor Object Reference") (OtherComp :type "PrimitiveComponent Object Reference") (OtherBodyIndex :type Integer) (bFromSweep :type Boolean) (SweepResult :type "HitResult Structure (by ref)"))
  (bind _marker (`self.Marker`))
  (`Widget.RemoveFromParent` (`self.Marker`))
  (`UserWidget.AddToViewport` _marker 0)
  (`/Game/DragonCore/UI/WDG_CompassMarker.InitMarker` _marker (`self.Marker Color`) "/Game/DragonCore/UI/MInst_ExclamationMarker.MInst_ExclamationMarker" self))

(fn `UserConstructionScript`
  (`MeshComponent.SetVectorParameterValueOnMaterials` (`self.StaticMesh`) "Color" (`KismetMathLibrary.Conv_LinearColorToVector` (`self.Marker Color`))))