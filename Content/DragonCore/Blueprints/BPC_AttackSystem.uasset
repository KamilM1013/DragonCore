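; Player attack component for a dragon character, handling a four-hit light combo, heavy tail swipe and rage attack that requires and spends full rage.
; Light input during an attack is buffered in SaveAttack, and SwordAttackCombo continues or resets the montage chain.
; Looping timers sphere-trace claw and tail points, alongside a single bite/AoE trace.
; Hits on Damageable actors deal damage with feedback effects; claw and tail hits also build rage.
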(event `EnhancedInput|/Game/ThirdPerson/Input/Actions/IA_OPAttack`
  (params (ActionValue :type Boolean) (ElapsedSeconds :type "Float (double-precision)") (TriggeredSeconds :type "Float (double-precision)") (InputAction :type "InputAction Object Reference" :default "/Game/ThirdPerson/Input/Actions/IA_OPAttack.IA_OPAttack"))
  (bind _bpc_playerstats (`/Game/ThirdPerson/Blueprints/BP_ThirdPersonCharacter.BPC_PlayerStats` (`self.Character`)))
  ;[0.05127 0.05127 0.05127] Rage Attack
  (:`Started`
    (if (>= (`/Game/DragonCore/Blueprints/BPC_PlayerStats.Current Rage` _bpc_playerstats) (`/Game/DragonCore/Blueprints/BPC_PlayerStats.Max Rage` _bpc_playerstats))
      (if (`self.canDoAction?`)
        (`self.OPAttack`)))))

(event `OPAttack`
  ;[0.05127 0.05127 0.05127] Rage Attack
  (if (not (`self.isAttacking?`))
    (set `self.isAttacking?` true)
    (switch `int` 0
      (:`0`
        (`self.OPAttackType 1`)
        (set `self.isAttacking?` false)))))

(event `OPAttackType 1`
  (bind _bpc_playerstats (`/Game/ThirdPerson/Blueprints/BP_ThirdPersonCharacter.BPC_PlayerStats` (`self.Character`)))
  ;[0.05127 0.05127 0.05127] Rage Attack
  (`/Engine/EditorBlueprintResources/StandardMacros.DoOnce` false :!label _label
    (:`Completed`
      (`KismetSystemLibrary.Delay` 0.1)
      (`|PlayMontage` (`self.CharacterMesh`) "/Game/DragonCore/PlayerCharacters/Noxturn/Animations/Montages/Attack/Anim_Nox_Attack_MagicWall_Montage.Anim_Nox_Attack_MagicWall_Montage"
        (:`then`
          (`/Game/DragonCore/Blueprints/BPC_PlayerStats.Decrease Rage` _bpc_playerstats (`/Game/DragonCore/Blueprints/BPC_PlayerStats.Max Rage` _bpc_playerstats))
          (goto _label :!via `Reset`))))))

(event `EnhancedInput|/Game/ThirdPerson/Input/Actions/IA_HeavyAttck`
  (params (ActionValue :type Boolean) (ElapsedSeconds :type "Float (double-precision)") (TriggeredSeconds :type "Float (double-precision)") (InputAction :type "InputAction Object Reference" :default "/Game/ThirdPerson/Input/Actions/IA_HeavyAttck.IA_HeavyAttck"))
  ;[0.05127 0.05127 0.05127] Heavy Attack
  (:`Started`
    (if (`self.canDoAction?`)
      (`self.HeavyATtack`))))

(event `HeavyAttack`
  ;[0.05127 0.05127 0.05127] Heavy Attack
  (if (not (`self.isAttacking?`))
    (set `self.isAttacking?` true)
    (switch `int` 0
      (:`0`
        (`self.CarryOutHeavyAttack`)
        (set `self.isAttacking?` false)))))

(event `CarryOutHeavyAttack`
  ;[0.05127 0.05127 0.05127] Heavy Attack
  (`/Engine/EditorBlueprintResources/StandardMacros.DoOnce` false :!label _label_2
    (:`Completed`
      (`KismetSystemLibrary.Delay` 0.1)
      (`|PlayMontage` (`self.CharacterMesh`) "/Game/DragonCore/PlayerCharacters/Noxturn/Animations/Montages/Attack/Anim_Nox_Attack_Tailswipe_Montage.Anim_Nox_Attack_Tailswipe_Montage"
        (:`OnCompleted`
          (goto _label_2 :!via `Reset`))
        (:`OnInterrupted`
          (goto _label_2 :!via `Reset`))))))

(event `self.ReceiveBeginPlay`
  ;[0.05127 0.05127 0.05127] Light Attack/ Combo System
  (bind _asbp_third_person_character (cast `/Game/ThirdPerson/Blueprints/BP_ThirdPersonCharacter` (`self.GetOwner`)))
  (set `self.Character` _asbp_third_person_character)
  (set `self.CharacterMesh` (`Character.Mesh` _asbp_third_person_character)))

(event `Attack 1`
  ;[0.05127 0.05127 0.05127] Light Attack/ Combo System
  ;;[0.05127 0.05127 0.05127] Attack 1
  (`/Engine/EditorBlueprintResources/StandardMacros.DoOnce` false :!label _label_3
    (:`Completed`
      (`KismetSystemLibrary.Delay` 0.1)
      (`|PlayMontage` (`self.CharacterMesh`) "/Game/DragonCore/PlayerCharacters/Noxturn/Animations/Montages/Attack/Anim_Nox_Attack_RightScratch_Montage.Anim_Nox_Attack_RightScratch_Montage"
        (:`then`
          (set `self.AttackIndex` 1)
          (goto _label_3 :!via `Reset`))))))

(event `EnhancedInput|/Game/ThirdPerson/Input/Actions/IA_LightAttack`
  (params (ActionValue :type Boolean) (ElapsedSeconds :type "Float (double-precision)") (TriggeredSeconds :type "Float (double-precision)") (InputAction :type "InputAction Object Reference" :default "/Game/ThirdPerson/Input/Actions/IA_LightAttack.IA_LightAttack"))
  ;[0.05127 0.05127 0.05127] Light Attack/ Combo System
  ;;[0.05127 0.05127 0.05127] Attack Input
  (:`Started`
    (if true
      (if (`self.canDoAction?`)
        (`self.SwordAttack`)))))

(event `Attack 2`
  ;[0.05127 0.05127 0.05127] Light Attack/ Combo System
  ;;[0.05127 0.05127 0.05127] Attack 2
  (`/Engine/EditorBlueprintResources/StandardMacros.DoOnce` false :!label _label_4
    (:`Completed`
      (`KismetSystemLibrary.Delay` 0.1)
      (`|PlayMontage` (`self.CharacterMesh`) "/Game/DragonCore/PlayerCharacters/Noxturn/Animations/Montages/Attack/Anim_Nox_Attack_LeftScratch_Montage.Anim_Nox_Attack_LeftScratch_Montage"
        (:`then`
          (set `self.AttackIndex` 2)
          (goto _label_4 :!via `Reset`))))))

(event `SwordAttack`
  ;[0.05127 0.05127 0.05127] Light Attack/ Combo System
  ;;[0.05127 0.05127 0.05127] Attack
  (if (`self.isAttacking?`)
    (set `self.saveAttack?` true)
    (else
      (set `self.isAttacking?` true)
      (switch `int` (`self.AttackIndex`) :!label _label_5
        (:`0`
          (`self.Attack 1`))
        (:`1`
          (`self.Attack 2`))
        (:`2`
          (`self.Attack 3`))
        (:`3`
          (`self.Attack 4`))))))

(event `Attack 3`
  ;[0.05127 0.05127 0.05127] Light Attack/ Combo System
  ;;[0.05127 0.05127 0.05127] Attack 3
  (`/Engine/EditorBlueprintResources/StandardMacros.DoOnce` false :!label _label_6
    (:`Completed`
      (`KismetSystemLibrary.Delay` 0.1)
      (`|PlayMontage` (`self.CharacterMesh`) "/Game/DragonCore/PlayerCharacters/Noxturn/Animations/Montages/Attack/Anim_Nox_Attack_RightWingPunch_Montage.Anim_Nox_Attack_RightWingPunch_Montage"
        (:`then`
          (set `self.AttackIndex` 3)
          (goto _label_6 :!via `Reset`))))))

(event `SwordAttackCombo`
  ;[0.05127 0.05127 0.05127] Light Attack/ Combo System
  ;;[0.05127 0.05127 0.05127] Combo Continue
  (if (`self.saveAttack?`)
    (set `self.saveAttack?` false)
    (goto _label_5)
    (else
      (`self.StopCombo`))))

(event `StopCombo`
  ;[0.05127 0.05127 0.05127] Light Attack/ Combo System
  ;;[0.05127 0.05127 0.05127] Stop Combo
  (set `self.isAttacking?` false)
  (set `self.AttackIndex` 0))

(event `Attack 4`
  ;[0.05127 0.05127 0.05127] Light Attack/ Combo System
  ;;[0.05127 0.05127 0.05127] Attack 4
  (`/Engine/EditorBlueprintResources/StandardMacros.DoOnce` false :!label _label_7
    (:`Completed`
      (`KismetSystemLibrary.Delay` 0.1)
      (`|PlayMontage` (`self.CharacterMesh`) "/Game/DragonCore/PlayerCharacters/Noxturn/Animations/Montages/Attack/Anim_Nox_Attack_Bite_Montage.Anim_Nox_Attack_Bite_Montage"
        (:`then`
          (set `self.AttackIndex` 4)
          (goto _label_7 :!via `Reset`))))))

(event `R_StartAttackTrace`
  ;[0.05127 0.05127 0.05127] Right_Swipe Trace
  (bind _returnvalue (`KismetSystemLibrary.K2_SetTimerDelegate` (delegate `R_AttackTraceLoop`) 0.001 true))
  (set `self.AttackTrace` _returnvalue))

(event `R_AttackTraceLoop`
  (bind _returnvalue (`self.GetOwner`))
  (bind _character (`self.Character`))
  ;[0.05127 0.05127 0.05127] Right_Swipe Trace
  (bind (_outhit _returnvalue_2) (`KismetSystemLibrary.SphereTraceSingle` :`Start` (`SceneComponent.K2_GetComponentLocation` (`/Game/ThirdPerson/Blueprints/BP_ThirdPersonCharacter.R_TopPoint` _character)) :`End` (`SceneComponent.K2_GetComponentLocation` (`/Game/ThirdPerson/Blueprints/BP_ThirdPersonCharacter.R_BottomPoint` _character)) :`Radius` 30.0 :`TraceChannel` "TraceTypeQuery1" :`DrawDebugType` "ForDuration" :`DrawTime` 0.2))
  (if _returnvalue_2
    (bind (_bblockinghit _binitialoverlap _time _distance _location _impactpoint _normal _impactnormal _physmat _hitactor) (`GameplayStatics.BreakHitResult` _outhit))
    (if (`Actor.ActorHasTag` _hitactor "Damageable")
      (bind _asmaster_enemy (cast `/Game/DragonCore/AI_Classes/Enemies/Master_Enemy` _hitactor)
        (:`then`
          (`AISense_Damage.ReportDamageEvent` _asmaster_enemy _returnvalue 0.0 (`Actor.K2_GetActorLocation` _returnvalue) _impactpoint))
        (:`CastFailed`
          _))
      (`GameplayStatics.ApplyDamage` _hitactor (`/Game/DragonCore/Blueprints/BPC_PlayerStats.Damage` (`/Game/ThirdPerson/Blueprints/BP_ThirdPersonCharacter.BPC_PlayerStats` (`self.Character`))))
      (`/Engine/EditorBlueprintResources/StandardMacros.DoOnce` false :!label _label_8
        (:`Completed`
          (`/Game/DragonCore/Blueprints/BPC_PlayerStats.Increase Rage` (`/Game/ThirdPerson/Blueprints/BP_ThirdPersonCharacter.BPC_PlayerStats` (`self.Character`)) 8.0)
          (`GameplayStatics.PlayWorldCameraShake` "/Game/DragonCore/Blueprints/BP_HitCameraShake.BP_HitCameraShake_C" _location 0.0 2000.0)
          (`self.PlayAttackHitSounds`)
          (`GameplayStatics.SpawnEmitterAtLocation` "/Game/DragonCore/VFX/Realistic_Starter_VFX_Pack_Vol2/Particles/Blood/P_Blood_Splat_Cone.P_Blood_Splat_Cone" _location (`KismetMathLibrary.MakeRotFromXY` _normal _normal) (0.4 0.4 0.4) true "AutoRelease")
          (`KismetSystemLibrary.Delay` 0.5)
          (goto _label_8 :!via `Reset`))))))

(event `R_StopAttackTrace`
  ;[0.05127 0.05127 0.05127] Right_Swipe Trace
  (`KismetSystemLibrary.K2_ClearAndInvalidateTimerHandle` (`self.AttackTrace`)))

(event `L_StartAttackTrace`
  ;[0.05127 0.05127 0.05127] Left_Swipe Trace
  (bind _returnvalue (`KismetSystemLibrary.K2_SetTimerDelegate` (delegate `L_AttackTraceLoop`) 0.001 true))
  (set `self.AttackTrace` _returnvalue))

(event `L_AttackTraceLoop`
  (bind _returnvalue (`self.GetOwner`))
  (bind _character (`self.Character`))
  ;[0.05127 0.05127 0.05127] Left_Swipe Trace
  (bind (_outhit _returnvalue_2) (`KismetSystemLibrary.SphereTraceSingle` :`Start` (`SceneComponent.K2_GetComponentLocation` (`/Game/ThirdPerson/Blueprints/BP_ThirdPersonCharacter.L_TopPoint` _character)) :`End` (`SceneComponent.K2_GetComponentLocation` (`/Game/ThirdPerson/Blueprints/BP_ThirdPersonCharacter.L_BottomPoint` _character)) :`Radius` 30.0 :`TraceChannel` "TraceTypeQuery1" :`DrawDebugType` "ForDuration" :`DrawTime` 0.2))
  (if _returnvalue_2
    (bind (_bblockinghit _binitialoverlap _time _distance _location _impactpoint _normal _impactnormal _physmat _hitactor) (`GameplayStatics.BreakHitResult` _outhit))
    (if (`Actor.ActorHasTag` _hitactor "Damageable")
      (bind _asmaster_enemy (cast `/Game/DragonCore/AI_Classes/Enemies/Master_Enemy` _hitactor)
        (:`then`
          (`AISense_Damage.ReportDamageEvent` _asmaster_enemy _returnvalue 0.0 (`Actor.K2_GetActorLocation` _returnvalue) _impactpoint))
        (:`CastFailed`
          _))
      (`GameplayStatics.ApplyDamage` _hitactor (`/Game/DragonCore/Blueprints/BPC_PlayerStats.Damage` (`/Game/ThirdPerson/Blueprints/BP_ThirdPersonCharacter.BPC_PlayerStats` (`self.Character`))))
      (`/Engine/EditorBlueprintResources/StandardMacros.DoOnce` false :!label _label_9
        (:`Completed`
          (`/Game/DragonCore/Blueprints/BPC_PlayerStats.Increase Rage` (`/Game/ThirdPerson/Blueprints/BP_ThirdPersonCharacter.BPC_PlayerStats` (`self.Character`)) 8.0)
          (`GameplayStatics.PlayWorldCameraShake` "/Game/DragonCore/Blueprints/BP_HitCameraShake.BP_HitCameraShake_C" _location 0.0 2000.0)
          (`self.PlayAttackHitSounds`)
          (`GameplayStatics.SpawnEmitterAtLocation` "/Game/DragonCore/VFX/Realistic_Starter_VFX_Pack_Vol2/Particles/Blood/P_Blood_Splat_Cone.P_Blood_Splat_Cone" _location (`KismetMathLibrary.MakeRotFromXY` _normal _normal) (0.4 0.4 0.4) true "AutoRelease")
          (`KismetSystemLibrary.Delay` 0.5)
          (goto _label_9 :!via `Reset`))))))

(event `L_StopAttackTrace`
  ;[0.05127 0.05127 0.05127] Left_Swipe Trace
  (`KismetSystemLibrary.K2_ClearAndInvalidateTimerHandle` (`self.AttackTrace`)))

(event `T_StartAttackTrace`
  ;[0.05127 0.05127 0.05127] Tail_Swipe Trace
  (bind _returnvalue (`KismetSystemLibrary.K2_SetTimerDelegate` (delegate `T_AttackTraceLoop`) 0.001 true))
  (set `self.AttackTrace` _returnvalue))

(event `T_AttackTraceLoop`
  (bind _returnvalue (`self.GetOwner`))
  (bind _character (`self.Character`))
  ;[0.05127 0.05127 0.05127] Tail_Swipe Trace
  (bind (_outhit _returnvalue_2) (`KismetSystemLibrary.SphereTraceSingle` :`Start` (`SceneComponent.K2_GetComponentLocation` (`/Game/ThirdPerson/Blueprints/BP_ThirdPersonCharacter.T_TopPoint` _character)) :`End` (`SceneComponent.K2_GetComponentLocation` (`/Game/ThirdPerson/Blueprints/BP_ThirdPersonCharacter.T_BottomPoint` _character)) :`Radius` 50.0 :`TraceChannel` "TraceTypeQuery1" :`DrawDebugType` "ForDuration" :`DrawTime` 0.2))
  (if _returnvalue_2
    (bind (_bblockinghit _binitialoverlap _time _distance _location _impactpoint _normal _impactnormal _physmat _hitactor) (`GameplayStatics.BreakHitResult` _outhit))
    (if (`Actor.ActorHasTag` _hitactor "Damageable")
      (bind _asmaster_enemy (cast `/Game/DragonCore/AI_Classes/Enemies/Master_Enemy` _hitactor)
        (:`then`
          (`AISense_Damage.ReportDamageEvent` _asmaster_enemy _returnvalue 0.0 (`Actor.K2_GetActorLocation` _returnvalue) _impactpoint))
        (:`CastFailed`
          _))
      (`GameplayStatics.ApplyDamage` _hitactor (+ (`/Game/DragonCore/Blueprints/BPC_PlayerStats.Damage` (`/Game/ThirdPerson/Blueprints/BP_ThirdPersonCharacter.BPC_PlayerStats` (`self.Character`))) 30.0))
      (`/Engine/EditorBlueprintResources/StandardMacros.DoOnce` false :!label _label_10
        (:`Completed`
          (`/Game/DragonCore/Blueprints/BPC_PlayerStats.Increase Rage` (`/Game/ThirdPerson/Blueprints/BP_ThirdPersonCharacter.BPC_PlayerStats` (`self.Character`)) 100.0)
          (`GameplayStatics.PlayWorldCameraShake` "/Game/DragonCore/Blueprints/BP_HitCameraShake.BP_HitCameraShake_C" _location 0.0 2000.0)
          (`self.PlayAttackHitSounds`)
          (`GameplayStatics.SpawnEmitterAtLocation` "/Game/DragonCore/VFX/Realistic_Starter_VFX_Pack_Vol2/Particles/Blood/P_Blood_Splat_Cone.P_Blood_Splat_Cone" _location (`KismetMathLibrary.MakeRotFromXY` _normal _normal) (0.4 0.4 0.4) true "AutoRelease")
          (`KismetSystemLibrary.Delay` 0.5)
          (goto _label_10 :!via `Reset`))))))

(event `T_StopAttackTrace`
  ;[0.05127 0.05127 0.05127] Tail_Swipe Trace
  (`KismetSystemLibrary.K2_ClearAndInvalidateTimerHandle` (`self.AttackTrace`)))

(event `SphereTrace`
  (bind _returnvalue (`self.GetOwner`))
  (bind _returnvalue_2 (`SceneComponent.K2_GetComponentLocation` (`/Game/ThirdPerson/Blueprints/BP_ThirdPersonCharacter.SphereTrace` (`self.Character`))))
  ;[0.05127 0.05127 0.05127] Sphere Trace (Bite/AoE)
  (bind (_outhit _returnvalue_3) (`KismetSystemLibrary.SphereTraceSingle` :`Start` _returnvalue_2 :`End` _returnvalue_2 :`Radius` 75.0 :`TraceChannel` "TraceTypeQuery1" :`DrawDebugType` "ForDuration" :`DrawTime` 0.2))
  (if _returnvalue_3
    (bind (_bblockinghit _binitialoverlap _time _distance _location _impactpoint _normal _impactnormal _physmat _hitactor) (`GameplayStatics.BreakHitResult` _outhit))
    (if (`Actor.ActorHasTag` _hitactor "Damageable")
      (bind _asmaster_enemy (cast `/Game/DragonCore/AI_Classes/Enemies/Master_Enemy` _returnvalue)
        (:`then`
          (`AISense_Damage.ReportDamageEvent` _asmaster_enemy _returnvalue 0.0 (`Actor.K2_GetActorLocation` _returnvalue) _impactpoint))
        (:`CastFailed`
          _))
      (`GameplayStatics.ApplyDamage` _hitactor 10.0)
      (`GameplayStatics.PlayWorldCameraShake` "/Game/DragonCore/Blueprints/BP_HitCameraShake.BP_HitCameraShake_C" _location 0.0 2000.0)
      (`self.PlayAttackHitSounds`)
      (`GameplayStatics.SpawnEmitterAtLocation` "/Game/DragonCore/VFX/Realistic_Starter_VFX_Pack_Vol2/Particles/Blood/P_Blood_Splat_Cone.P_Blood_Splat_Cone" _location (`KismetMathLibrary.MakeRotFromXY` _normal _normal) (0.4 0.4 0.4) true "AutoRelease"))))

(event `PlayAttackHitSounds`
  ;[0.05127 0.05127 0.05127] Play Attack Hit Sounds
  (`GameplayStatics.PlaySoundAtLocation` "/Game/DragonCore/Audio/Hits/MS_AttackHits.MS_AttackHits" (`Actor.K2_GetActorLocation` (`self.GetOwner`)) (struct) 1.0 1.0 0.0 null null null null))