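; BP_Location is a trigger volume actor that shows an area name on the player's HUD compass.
; When BP_ThirdPersonCharacter begins overlapping the Trigger, it writes its Location value to the compass text and plays the FadeIn animation.
; Ending the overlap plays the same animation in reverse to fade the name out, leaving the text itself in place.
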(event `self.Trigger.OnComponentBeginOverlap`
  (params (OverlappedComponent :type "PrimitiveComponent Object Reference") (OtherActor :type "Actor Object Reference") (OtherComp :type "PrimitiveComponent Object Reference") (OtherBodyIndex :type Integer) (bFromSweep :type Boolean) (SweepResult :type "HitResult Structure (by ref)"))
  ;[0.05127 0.05127 0.05127] Fade in location name when stepping into boundaries
  (bind _asbp_third_person_character (cast `/Game/ThirdPerson/Blueprints/BP_ThirdPersonCharacter` OtherActor))
  (bind _hud_compass (`/Game/ThirdPerson/Blueprints/BP_ThirdPersonCharacter.HUD Compass` _asbp_third_person_character))
  (set `TextBlock.Text` (`self.Location`) (`/Game/DragonCore/HUD/Widgets/WB_Compass.Location` _hud_compass))
  (`UserWidget.PlayAnimation` _hud_compass (`/Game/DragonCore/HUD/Widgets/WB_Compass.FadeIn` _hud_compass) 0.0 1 "Forward" 1.0 false))

(event `self.Trigger.OnComponentEndOverlap`
  (params (OverlappedComponent :type "PrimitiveComponent Object Reference") (OtherActor :type "Actor Object Reference") (OtherComp :type "PrimitiveComponent Object Reference") (OtherBodyIndex :type Integer))
  ;[0.05127 0.05127 0.05127] Fade out location name when stepping out of boundaries
  (bind _asbp_third_person_character (cast `/Game/ThirdPerson/Blueprints/BP_ThirdPersonCharacter` OtherActor))
  (bind _hud_compass (`/Game/ThirdPerson/Blueprints/BP_ThirdPersonCharacter.HUD Compass` _asbp_third_person_character))
  (`UserWidget.PlayAnimation` _hud_compass (`/Game/DragonCore/HUD/Widgets/WB_Compass.FadeIn` _hud_compass) 0.0 1 "Reverse" 1.0 false))

(fn `UserConstructionScript`)