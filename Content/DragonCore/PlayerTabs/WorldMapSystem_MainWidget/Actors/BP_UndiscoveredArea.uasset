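; World map actor that marks an undiscovered area and detects when a player enters it.
; Construction Script sizes AreaSphere from AreaRadius and DiscoverSphere from that radius plus an additional discovery margin.
; The first DiscoverSphere overlap by an actor with BPC_WorldMap_ActivatePlayerTabs passes this area to that component's OnDiscoveredArea.
; A separate OnDiscovered event destroys the actor.
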(event `self.DiscoverSphere.OnComponentBeginOverlap`
  (params (OverlappedComponent :type "PrimitiveComponent Object Reference") (OtherActor :type "Actor Object Reference") (OtherComp :type "PrimitiveComponent Object Reference") (OtherBodyIndex :type Integer) (bFromSweep :type Boolean) (SweepResult :type "HitResult Structure (by ref)"))
  (bind _returnvalue (`self.GetComponentByClass` OtherActor "/Game/DragonCore/PlayerTabs/WorldMapSystem_MainWidget/Actors/BPC_WorldMap_ActivatePlayerTabs.BPC_WorldMap_ActivatePlayerTabs_C"))
  ;[0.05127 0.05127 0.05127] Destroy actor when entering discover sphere; trigger event in world map component
  (`/Engine/EditorBlueprintResources/StandardMacros.IsValid` _returnvalue
    (:`Is Valid`
      (`/Engine/EditorBlueprintResources/StandardMacros.DoOnce` false
        (:`Completed`
          (`/Game/DragonCore/PlayerTabs/WorldMapSystem_MainWidget/Actors/BPC_WorldMap_ActivatePlayerTabs.OnDiscoveredArea` _returnvalue self))))))

(event `OnDiscovered`
  ;[0.05127 0.05127 0.05127] Destroy actor when entering discover sphere; trigger event in world map component
  (`self.K2_DestroyActor`))

(fn `UserConstructionScript`
  (`SphereComponent.SetSphereRadius` (`self.AreaSphere`) (`self.AreaRadius`) false)
  (`SphereComponent.SetSphereRadius` (`self.DiscoverSphere`) (+ (`self.AdditionalDiscoverRadius`) (`self.AreaRadius`)) false))