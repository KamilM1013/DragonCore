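; Player equipment component, in a deprecated folder, that picks up world items and stores their data.
; On BeginPlay it caches the owning third-person character's camera and attack system.
; The interact input sphere-traces forward from the camera, appends a hit BP_Item's data to ItemSlots, then destroys the actor.
; An unconnected graph holds a player-tabs menu toggle that blocks actions and movement and nearly freezes time.
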(event `self.ReceiveBeginPlay`
  ;[0.05127 0.05127 0.05127] Event Begin Play
  (bind _asbp_third_person_character (cast `/Game/ThirdPerson/Blueprints/BP_ThirdPersonCharacter` (`self.GetOwner`)))
  (set `self.Follow Camera` (`/Game/ThirdPerson/Blueprints/BP_ThirdPersonCharacter.FollowCamera` _asbp_third_person_character))
  (set `self.BPC Attack System` (`/Game/ThirdPerson/Blueprints/BP_ThirdPersonCharacter.BPC_AttackSystem` _asbp_third_person_character))
  (set `self.Player Character` _asbp_third_person_character))

(event `EnhancedInput|/Game/ThirdPerson/Input/Actions/IA_Interact`
  (params (ActionValue :type Boolean) (ElapsedSeconds :type "Float (double-precision)") (TriggeredSeconds :type "Float (double-precision)") (InputAction :type "InputAction Object Reference" :default "/Game/ThirdPerson/Input/Actions/IA_Interact.IA_Interact"))
  (bind _follow_camera (`self.Follow Camera`))
  (bind _returnvalue (`SceneComponent.K2_GetComponentLocation` _follow_camera))
  ;[0.05127 0.05127 0.05127] PickUp Trace
  (:`Started`
    (bind (_outhit _returnvalue_2) (`KismetSystemLibrary.SphereTraceSingleForObjects` _returnvalue (+ _returnvalue (* (`KismetMathLibrary.GetForwardVector` (`SceneComponent.K2_GetComponentRotation` _follow_camera)) 1000.0)) 15.0 (`|MakeArray` "ObjectTypeQuery2" :!type "EObjectTypeQuery Enum")))
    (if _returnvalue_2
      (bind _asbp_item (cast `/Game/DragonCore/PlayerTabs/Deprecated_EquipmentSystem/BP_Item` (`.HitActor` (`GameplayStatics.BreakHitResult` _outhit))))
      (`self.AddItem` (`/Game/DragonCore/PlayerTabs/Deprecated_EquipmentSystem/BP_Item.ItemData` _asbp_item))
      (`Actor.K2_DestroyActor` _asbp_item))))

(event `EnhancedInput|/Game/ThirdPerson/Input/Actions/IA_PlayerTabs`
  (params (ActionValue :type Boolean) (ElapsedSeconds :type "Float (double-precision)") (TriggeredSeconds :type "Float (double-precision)") (InputAction :type "InputAction Object Reference" :default "/Game/ThirdPerson/Input/Actions/IA_PlayerTabs.IA_PlayerTabs"))
  ;[0.05127 0.05127 0.05127] Inventory Menu Panel
  ;;[0.05127 0.05127 0.05127] Gear
)

(fn `AddItem`
  (params (NewItem :type "/Game/DragonCore/PlayerTabs/Deprecated_EquipmentSystem/S_Slots Structure (by ref)"))
  (`KismetArrayLibrary.Array_Add` (`self.ItemSlots`) NewItem))