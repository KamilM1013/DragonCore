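; Interactable loot chest that grants a random common or rare gear item from the player's BPC_GearSystem.
; BeginPlay either idles with an interaction prompt or, if already opened, removes the prompt and plays the open animation.
; CallOpenChest runs once, playing effects, sending and removing a pooled item, and registering the chest as opened.
; It shows a timed item pop-up, then destroys the coin burst.
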(event `self.ReceiveBeginPlay`
  (if (not (`self.openedChest`))
    (`SkeletalMeshComponent.PlayAnimation` (`self.Chest`) "/Game/DragonCore/Assets/Chest/chest_Anim_ChestArmature_Idle.chest_Anim_ChestArmature_Idle" true)
    (bind _aswb_interaction (cast `/Game/DragonCore/PlayerTabs/GearSystem/Widgets/WB_Interaction` (`WidgetComponent.GetWidget` (`self.Interaction`))))
    (bind _output_get (set `self.WB Interaction` _aswb_interaction))
    (`/Game/DragonCore/PlayerTabs/GearSystem/Widgets/WB_Interaction.UpdateText` _output_get (`self.InteractableType`))
    (else
      (`ActorComponent.K2_DestroyComponent` (`self.Interaction`))
      (`ActorComponent.K2_DestroyComponent` (`self.InteractCall`))
      (`SkeletalMeshComponent.PlayAnimation` (`self.Chest`) "/Game/DragonCore/Assets/Chest/chest_Anim_ChestArmature_Open.chest_Anim_ChestArmature_Open" false))))

(event `/Game/DragonCore/PlayerTabs/GearSystem/BPI_Inventory.CallOpenChest`
  (bind _commonandrareitems (`/Game/DragonCore/PlayerTabs/GearSystem/BPC_GearSystem.CommonAndRareItems` (`self.Get BPC Gear Ref`)))
  (if (not (`self.openedChest`))
    (`/Engine/EditorBlueprintResources/StandardMacros.DoOnce` false
      (:`Completed`
        (`GameplayStatics.PlaySound2D` "/Game/DragonCore/Audio/Meditate.Meditate" 1.0 1.0 0.0 null null)
        (`ActorComponent.K2_DestroyComponent` (`self.InteractCall`))
        (`SkeletalMeshComponent.PlayAnimation` (`self.Chest`) "/Game/DragonCore/Assets/Chest/chest_Anim_ChestArmature_Open.chest_Anim_ChestArmature_Open" false)
        (`ActorComponent.Activate` (`self.CoinBurst`) false)
        (bind _output_get (set `self.RandomItem` (`KismetArrayLibrary.Array_Random` _commonandrareitems)))
        (`/Game/DragonCore/PlayerTabs/GearSystem/BPC_GearSystem.SendRandomItem` (`self.Get BPC Gear Ref`) _output_get)
        (`KismetArrayLibrary.Array_RemoveItem` _commonandrareitems _output_get)
        (set `self.openedChest` true)
        (bind _returnvalue (`|CreateWidget` "/Game/DragonCore/PlayerTabs/GearSystem/Widgets/WB_ChestPopUp.WB_ChestPopUp_C"))
        (bind _output_get_2 (set `self.ChestPopUp` _returnvalue))
        (`/Game/DragonCore/PlayerTabs/GearSystem/Widgets/WB_ChestPopUp.CallPopup` _output_get_2 _output_get)
        (`UserWidget.AddToViewport` _output_get_2 0)
        (`KismetArrayLibrary.Array_Add` (`/Game/DragonCore/PlayerTabs/GearSystem/BPC_GearSystem.openedChests` (`self.Get BPC Gear Ref`)) self)
        (`KismetSystemLibrary.Delay` 3.0)
        (`Widget.RemoveFromParent` (`self.ChestPopUp`))
        (`KismetSystemLibrary.Delay` 2.0)
        (`ActorComponent.K2_DestroyComponent` (`self.CoinBurst`))))))

(fn `UserConstructionScript`)