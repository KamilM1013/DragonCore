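; Interactable shrine actor where the player meditates to restore health.
; On BeginPlay it sets its interaction widget's text from the interactable type.
; CallMeditate starts particles and a sound, hides the prompt, messages the player's gear component to play the meditate animation and increases health by MaxHealth through the stats component.
; A DoOnce blocks repeat use until a delay ends, when particles stop and the prompt returns.
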(event `self.ReceiveBeginPlay`
  (bind _aswb_interaction (cast `/Game/DragonCore/PlayerTabs/GearSystem/Widgets/WB_Interaction` (`WidgetComponent.GetWidget` (`self.Interaction`))))
  (bind _output_get (set `self.WB Interaction` _aswb_interaction))
  (`/Game/DragonCore/PlayerTabs/GearSystem/Widgets/WB_Interaction.UpdateText` _output_get (`self.InteractableType`)))

(event `/Game/DragonCore/PlayerTabs/GearSystem/BPI_Inventory.CallMeditate`
  (bind _bpc_playerstats (`self.Get BPC PlayerStats Ref`))
  (`/Engine/EditorBlueprintResources/StandardMacros.DoOnce` false :!label _label
    (:`Completed`
      (`ActorComponent.Activate` (`self.ParticleSystem`) false)
      (`GameplayStatics.PlaySound2D` "/Game/DragonCore/Audio/harpsweep.harpsweep" 1.0 1.0 0.0 null null)
      (`SceneComponent.SetVisibility` (`self.Interaction`) false false)
      (message `/Game/DragonCore/PlayerTabs/GearSystem/BPI_Gear.MeditateAnim` (`self.Get BPC Gear Ref`))
      (`/Game/DragonCore/Combat/BPC_PlayerStats.Increase Health` _bpc_playerstats (`/Game/DragonCore/Combat/BPC_PlayerStats.Max Health` _bpc_playerstats))
      (`KismetSystemLibrary.Delay` 9.0)
      (`ActorComponent.Deactivate` (`self.ParticleSystem`))
      (`SceneComponent.SetVisibility` (`self.Interaction`) true false)
      (goto _label :!via `Reset`))))

(fn `UserConstructionScript`)