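; Epic loot chest that grants a random item from the gear system's EpicItems list.
; On BeginPlay it loops an idle animation and sets its interaction widget text from the interactable type.
; CallOpenChest runs once, removing the interact component, playing the open animation and coin burst, then sending the item and removing it from the list.
; Both particle components are destroyed five seconds later.
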(event `self.ReceiveBeginPlay`
  (`SkeletalMeshComponent.PlayAnimation` (`self.Chest`) "/Game/DragonCore/Assets/Chest/chest_Anim_ChestArmature_Idle.chest_Anim_ChestArmature_Idle" true)
  (bind _aswb_interaction (cast `/Game/DragonCore/PlayerTabs/GearSystem/Widgets/WB_Interaction` (`WidgetComponent.GetWidget` (`self.Interaction`))))
  (bind _output_get (set `self.WB Interaction` _aswb_interaction))
  (`/Game/DragonCore/PlayerTabs/GearSystem/Widgets/WB_Interaction.UpdateText` _output_get (`self.InteractableType`)))

(event `/Game/DragonCore/PlayerTabs/GearSystem/BPI_Inventory.CallOpenChest`
  (bind _epicitems (`/Game/DragonCore/PlayerTabs/GearSystem/BPC_GearSystem.EpicItems` (`self.Get BPC Gear Ref`)))
  (`/Engine/EditorBlueprintResources/StandardMacros.DoOnce` false
    (:`Completed`
      (`ActorComponent.K2_DestroyComponent` (`self.InteractCall`))
      (`ActorComponent.Deactivate` (`self.ParticleSystem`))
      (`SkeletalMeshComponent.PlayAnimation` (`self.Chest`) "/Game/DragonCore/Assets/Chest/chest_Anim_ChestArmature_Open.chest_Anim_ChestArmature_Open" false)
      (`ActorComponent.Activate` (`self.CoinBurst`) false)
      (bind _output_get (set `self.RandomItem` (`KismetArrayLibrary.Array_Random` _epicitems)))
      (`/Game/DragonCore/PlayerTabs/GearSystem/BPC_GearSystem.SendRandomItem` (`self.Get BPC Gear Ref`) _output_get)
      (`KismetArrayLibrary.Array_RemoveItem` _epicitems _output_get)
      (`KismetSystemLibrary.Delay` 5.0)
      (`ActorComponent.K2_DestroyComponent` (`self.ParticleSystem`))
      (`ActorComponent.K2_DestroyComponent` (`self.CoinBurst`)))))

(fn `UserConstructionScript`)