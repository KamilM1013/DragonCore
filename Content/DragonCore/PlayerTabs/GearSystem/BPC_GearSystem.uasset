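; Player character component that manages the gear inventory, equipment slots and potion use.
; Interact moves overlapping pickups into a class-based inventory, dropping spawns items ahead of the player, and the I key toggles a sorted inventory widget.
; Slot setters store equipped classes and swap body-part skeletal meshes from class defaults, then call an empty UpdateInventory.
; Consumables add their modifier to health or rage in player stats.
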(event `self.ReceiveBeginPlay`
  ;[0.05127 0.05127 0.05127] Event Begin Play
  (bind _asbp_third_person_character (cast `/Game/ThirdPerson/Blueprints/BP_ThirdPersonCharacter` (`self.GetOwner`)))
  (bind _output_get (set `self.Player Character` _asbp_third_person_character))
  (set `self.BPC Attack System` (`/Game/ThirdPerson/Blueprints/BP_ThirdPersonCharacter.BPC_AttackSystem` _output_get)))

(event `Initiate`
  (params (Target :type "Actor Object Reference"))
  ;[0.05127 0.05127 0.05127] Initiate
  (`|ExecutionSequence`))

(event `Key|I`
  (params (Key :type "Key Structure"))
  (:`Pressed`
    (`/Engine/EditorBlueprintResources/StandardMacros.FlipFlop`
      (:`A`
        (`self.ShowSortedItems`))
      (:`B`
        (`self.HideSortedItems`)))))

(event `SpawnItems`
  (params (Class :type "Actor Class Reference") (SpawnTransform :type "Transform Structure"))
  ;[0.05127 0.05127 0.05127] Spawn Item after dropping from Inventory (Not using)
  (`|SpawnActorFromClass` Class SpawnTransform "AdjustIfPossibleButAlwaysSpawn" "OverrideRootScale" null null))

(event `/Game/DragonCore/PlayerTabs/GearSystem/BPI_Gear.SpawnItem`
  (params (ItemToSpawn :type "/Game/DragonCore/PlayerTabs/GearSystem/BP_MasterItem Class Reference") (SpawnTransform :type "Transform Structure"))
  ;[0.05127 0.05127 0.05127] Spawn Item after dropping from Inventory (Not using)
)

(event `DestroyActor`
  (params (ActorToDestroy :type "Actor Object Reference"))
  ;[0.05127 0.05127 0.05127] Spawn Item after dropping from Inventory (Not using)
  (`Actor.K2_DestroyActor` ActorToDestroy))

(event `EnhancedInput|/Game/ThirdPerson/Input/Actions/IA_Interact`
  (params (ActionValue :type Boolean) (ElapsedSeconds :type "Float (double-precision)") (TriggeredSeconds :type "Float (double-precision)") (InputAction :type "InputAction Object Reference" :default "/Game/ThirdPerson/Input/Actions/IA_Interact.IA_Interact"))
  ;[0.05127 0.05127 0.05127] Interact
  (:`Started`
    (`self.TryPickupItem`)))

(event `SetHeadWear`
  (params (EquippedHeadWear :type "/Game/DragonCore/PlayerTabs/GearSystem/BP_MasterItem Class Reference"))
  ;[0.05127 0.05127 0.05127] If creating new widget everytime when you open it; use these events to set the equipped slots, otherwise they reset when you close the widget
  (set `self.EquippedHeadWear` EquippedHeadWear)
  (`self.OnEquippedHeadWear`)
  (`self.UpdateInventory` :!label _label))

(event `SetFrontBraces`
  (params (EquippedFrontBraces :type "/Game/DragonCore/PlayerTabs/GearSystem/BP_MasterItem Class Reference"))
  ;[0.05127 0.05127 0.05127] If creating new widget everytime when you open it; use these events to set the equipped slots, otherwise they reset when you close the widget
  (set `self.EquippedFrontBraces` EquippedFrontBraces)
  (`self.OnEquippedFrontBraces`)
  (goto _label))

(event `SetBackBraces`
  (params (EquippedBackBraces :type "/Game/DragonCore/PlayerTabs/GearSystem/BP_MasterItem Class Reference"))
  ;[0.05127 0.05127 0.05127] If creating new widget everytime when you open it; use these events to set the equipped slots, otherwise they reset when you close the widget
  (set `self.EquippedBackBraces` EquippedBackBraces)
  (`self.OnEquippedBackBraces`)
  (goto _label))

(event `SetNeckWear`
  (params (EquippedNeckWear :type "/Game/DragonCore/PlayerTabs/GearSystem/BP_MasterItem Class Reference"))
  ;[0.05127 0.05127 0.05127] If creating new widget everytime when you open it; use these events to set the equipped slots, otherwise they reset when you close the widget
  (set `self.EquippedNeckWear` EquippedNeckWear)
  (`self.OnEquippedNeckWear`)
  (goto _label))

(event `SetOutfit`
  (params (EquippedOutfit :type "/Game/DragonCore/PlayerTabs/GearSystem/BP_MasterItem Class Reference"))
  ;[0.05127 0.05127 0.05127] If creating new widget everytime when you open it; use these events to set the equipped slots, otherwise they reset when you close the widget
  (set `self.EquippedOutfit` EquippedOutfit)
  (`self.OnEquippedOutfit`)
  (goto _label))

(event `SetTailWear`
  (params (EquippedTailWear :type "/Game/DragonCore/PlayerTabs/GearSystem/BP_MasterItem Class Reference"))
  ;[0.05127 0.05127 0.05127] If creating new widget everytime when you open it; use these events to set the equipped slots, otherwise they reset when you close the widget
  (set `self.EquippedTailWear` EquippedTailWear)
  (`self.OnEquippedTailWear`)
  (goto _label))

(event `SetConsumable`
  (params (EquippedConsumable :type "/Game/DragonCore/PlayerTabs/GearSystem/BP_MasterItem Class Reference"))
  (set `self.EquippedConsumable` EquippedConsumable))

(event `UseConsumable`
  (bind _playerstats_ref (`self.Get PlayerStats Ref`))
  (bind (_item_name _description _itemimage _itemmesh _usephysics _userotatingmovement_ _maxstack _itemrarity _offense _defense _sellvalue _itemlevel _itemtype _equipsocket _unequipsocket _skeletalmesh _consumabletype _consumablemodifier) (defaults `Object` (`self.EquippedConsumable`)))
  (switch `/Game/DragonCore/PlayerTabs/GearSystem/E_ConsumableType` _consumabletype
    (:`NewEnumerator1`
      (set `/Game/DragonCore/Blueprints/BPC_PlayerStats.Current Health` (+ (`/Game/DragonCore/Blueprints/BPC_PlayerStats.Current Health` _playerstats_ref) _consumablemodifier) _playerstats_ref))
    (:`NewEnumerator2`
      (set `/Game/DragonCore/Blueprints/BPC_PlayerStats.Current Rage` (+ (`/Game/DragonCore/Blueprints/BPC_PlayerStats.Current Rage` _playerstats_ref) _consumablemodifier) _playerstats_ref))))

(fn `AddItemToInventory`
  (params (NewItem :type "/Game/DragonCore/PlayerTabs/GearSystem/BP_MasterItem Object Reference (by ref)"))
  (bind _wb_sorteditems (`self.WB_SortedItems`))
  (`KismetArrayLibrary.Array_Add` (`self.Inventory`) (`GameplayStatics.GetObjectClass` NewItem))
  (`/Engine/EditorBlueprintResources/StandardMacros.IsValid` _wb_sorteditems
    (:`Is Valid`
      (`/Game/DragonCore/PlayerTabs/GearSystem/Widgets/WB_SortedItemsInventory.Update` _wb_sorteditems (`self.Inventory`) "NewEnumerator0"))
    (:`Is Not Valid`
      _))
  (`GameplayStatics.PlaySound2D` "/Game/RunesSystem/Sound/SFX_Shop_Click.SFX_Shop_Click" 1.0 1.0 0.0 null null))

(fn `DestroyItem`
  (params (ItemToDestroy :type "/Game/DragonCore/PlayerTabs/GearSystem/BP_MasterItem Class Reference") (SlotType :type "/Game/DragonCore/PlayerTabs/GearSystem/E_ItemType Enum" :default "NewEnumerator0"))
  (locals (DropPosition :type "Transform Structure"))
  (bind _inventory (`self.Inventory`))
  (`KismetArrayLibrary.Array_Remove` _inventory (`KismetArrayLibrary.Array_Find` _inventory ItemToDestroy))
  (`/Game/DragonCore/PlayerTabs/GearSystem/Widgets/WB_SortedItemsInventory.Update` (`self.WB_SortedItems`) (`self.Inventory`) SlotType))

(fn `DropItem`
  (params (ItemToSpawn :type "/Game/DragonCore/PlayerTabs/GearSystem/BP_MasterItem Class Reference"))
  (locals (DropPosition :type "Transform Structure"))
  (bind _returnvalue (`KismetMathLibrary.RandomFloatInRange` -75.0 75.0))
  (bind _player_character (`self.Player Character`))
  (bind _inventory (`self.Inventory`))
  (set `local.DropPosition` (`KismetMathLibrary.Conv_VectorToTransform` (+ (+ (`Actor.K2_GetActorLocation` _player_character) (* (`KismetMathLibrary.GetForwardVector` (`Actor.K2_GetActorRotation` _player_character)) (`self.Item Drop Distance`))) (`KismetMathLibrary.MakeVector` _returnvalue _returnvalue))))
  (`self.SpawnItems` ItemToSpawn (`local.DropPosition`))
  (`KismetArrayLibrary.Array_Remove` _inventory (`KismetArrayLibrary.Array_Find` _inventory ItemToSpawn))
  (`/Game/DragonCore/PlayerTabs/GearSystem/Widgets/WB_SortedItemsInventory.Update` (`self.WB_SortedItems`) (`self.Inventory`) "NewEnumerator0"))

(fn `HideSortedItems`
  (bind _wb_sorteditems (`self.WB_SortedItems`))
  (`/Engine/EditorBlueprintResources/StandardMacros.IsValid` _wb_sorteditems
    (:`Is Valid`
      (`Widget.RemoveFromParent` _wb_sorteditems))))

(fn `OnEquippedBackBraces`
  (`SkeletalMeshComponent.SetSkeletalMeshAsset` (`/Game/ThirdPerson/Blueprints/BP_ThirdPersonCharacter.HindLegs` (`self.Player Character`)) (`.SkeletalMesh` (defaults `Object` (`self.EquippedBackBraces`)))))

(fn `OnEquippedFrontBraces`
  (`SkeletalMeshComponent.SetSkeletalMeshAsset` (`/Game/ThirdPerson/Blueprints/BP_ThirdPersonCharacter.FrontLegs` (`self.Player Character`)) (`.SkeletalMesh` (defaults `Object` (`self.EquippedFrontBraces`)))))

(fn `OnEquippedHeadWear`
  (`SkeletalMeshComponent.SetSkeletalMeshAsset` (`/Game/ThirdPerson/Blueprints/BP_ThirdPersonCharacter.Head` (`self.Player Character`)) (`.SkeletalMesh` (defaults `Object` (`self.EquippedHeadWear`)))))

(fn `OnEquippedNeckWear`
  (`SkeletalMeshComponent.SetSkeletalMeshAsset` (`/Game/ThirdPerson/Blueprints/BP_ThirdPersonCharacter.Neck` (`self.Player Character`)) (`.SkeletalMesh` (defaults `Object` (`self.EquippedNeckWear`)))))

(fn `OnEquippedOutfit`
  (`SkeletalMeshComponent.SetSkeletalMeshAsset` (`Character.Mesh` (`self.Player Character`)) (`.SkeletalMesh` (defaults `Object` (`self.EquippedOutfit`)))))

(fn `OnEquippedTailWear`
  (`SkeletalMeshComponent.SetSkeletalMeshAsset` (`/Game/ThirdPerson/Blueprints/BP_ThirdPersonCharacter.Tail` (`self.Player Character`)) (`.SkeletalMesh` (defaults `Object` (`self.EquippedTailWear`)))))

(fn `ShowSortedItems`
  (bind _returnvalue (`|CreateWidget` "/Game/DragonCore/PlayerTabs/GearSystem/Widgets/WB_SortedItemsInventory.WB_SortedItemsInventory_C" (`GameplayStatics.GetPlayerController` 0)))
  (bind _output_get (set `self.WB_SortedItems` _returnvalue))
  (`UserWidget.AddToViewport` _output_get 0)
  (`/Game/DragonCore/PlayerTabs/GearSystem/Widgets/WB_SortedItemsInventory.Update` _output_get (`self.Inventory`) "NewEnumerator0"))

(fn `TryPickupItem`
  (bind _itemtopickup (`self.ItemToPickup`))
  (bind _overlappingitems (`self.OverlappingItems`))
  (if (> (`KismetArrayLibrary.Array_Length` (`self.OverlappingItems`)) 0)
    (`self.AddItemToInventory` _itemtopickup)
    (`KismetArrayLibrary.Array_RemoveItem` _overlappingitems _itemtopickup)
    (`self.DestroyActor` _itemtopickup)
    (if (> (`KismetArrayLibrary.Array_Length` (`self.OverlappingItems`)) 0)
      (set `self.ItemToPickup` (`KismetArrayLibrary.Array_Random` _overlappingitems)))))

(fn `UpdateInventory`)