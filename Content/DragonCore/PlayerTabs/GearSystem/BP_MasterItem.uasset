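; Base pickup actor for the gear system, which an overlapping actor with a gear component can collect.
; On overlap it either adds itself to the inventory and destroys itself (auto-pickup), or registers as the item to pick up and shows its interaction prompt.
; Leaving deregisters it, hiding the prompt only when no overlapping items remain.
; The construction script enables physics, or otherwise removes rotating movement when unused.
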(event `self.ReceiveBeginPlay`
  (`SceneComponent.SetVisibility` (`self.Interaction`) false false))

(event `self.InteractCall.OnComponentBeginOverlap`
  (params (OverlappedComponent :type "PrimitiveComponent Object Reference") (OtherActor :type "Actor Object Reference") (OtherComp :type "PrimitiveComponent Object Reference") (OtherBodyIndex :type Integer) (bFromSweep :type Boolean) (SweepResult :type "HitResult Structure (by ref)"))
  (bind _returnvalue (`self.GetComponentByClass` OtherActor "/Game/DragonCore/PlayerTabs/GearSystem/BPC_GearSystem.BPC_GearSystem_C"))
  (if (`KismetSystemLibrary.DoesImplementInterface` _returnvalue "/Game/DragonCore/PlayerTabs/GearSystem/BPI_Gear.BPI_Gear_C")
    (if (`/Game/DragonCore/PlayerTabs/GearSystem/BPC_GearSystem.AutoPickup` _returnvalue)
      (`/Game/DragonCore/PlayerTabs/GearSystem/BPC_GearSystem.AddItemToInventory` _returnvalue self)
      (`self.K2_DestroyActor`)
      (else
        (`KismetArrayLibrary.Array_Add` (`/Game/DragonCore/PlayerTabs/GearSystem/BPC_GearSystem.OverlappingItems` _returnvalue) self)
        (set `/Game/DragonCore/PlayerTabs/GearSystem/BPC_GearSystem.ItemToPickup` self _returnvalue)
        (`SceneComponent.SetVisibility` (`self.Interaction`) true false)))))

(event `self.InteractCall.OnComponentEndOverlap`
  (params (OverlappedComponent :type "PrimitiveComponent Object Reference") (OtherActor :type "Actor Object Reference") (OtherComp :type "PrimitiveComponent Object Reference") (OtherBodyIndex :type Integer))
  (bind _overlappingitems (`/Game/DragonCore/PlayerTabs/GearSystem/BPC_GearSystem.OverlappingItems` (`self.GetComponentByClass` OtherActor "/Game/DragonCore/PlayerTabs/GearSystem/BPC_GearSystem.BPC_GearSystem_C")))
  (`KismetArrayLibrary.Array_RemoveItem` _overlappingitems self)
  (if (not (> (`KismetArrayLibrary.Array_Length` _overlappingitems) 0))
    (`SceneComponent.SetVisibility` (`self.Interaction`) false false)))

(fn `UserConstructionScript`
  (bind _staticmesh (`self.StaticMesh`))
  (if (`self.usePhysics?`)
    (`PrimitiveComponent.SetSimulatePhysics` _staticmesh true)
    (`PrimitiveComponent.SetCollisionEnabled` _staticmesh "QueryAndPhysics")
    (elif (not (`self.useRotatingMovement?`))
      (`ActorComponent.K2_DestroyComponent` (`self.RotatingMovement`)))))