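; Point of interest actor for the world map and compass, which starts undiscovered and is discovered when the player gets close.
; A SeeDistance sphere shows and hides its compass marker widget, created at BeginPlay with an undiscovered material.
; Entering DiscoverRange switches the marker to its type material and notifies the overlapper's BPC_WorldMap once; OnDiscovered destroys that sphere.
; Construction script sizes both spheres, and GetMapIconData supplies a question-mark map icon.
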(event `self.ReceiveBeginPlay`
  (bind _marker (`self.Marker`))
  (bind _asbp_third_person_character (cast `/Game/ThirdPerson/Blueprints/BP_ThirdPersonCharacter` (`GameplayStatics.GetPlayerCharacter` 0)))
  (set `self.Player` _asbp_third_person_character)
  (`KismetSystemLibrary.Delay` 0.2)
  (bind _returnvalue (`|CreateWidget` "/Game/DragonCore/HUD/Widgets/WDG_CompassMarker.WDG_CompassMarker_C"))
  (set `self.Marker` _returnvalue)
  (`UserWidget.AddToViewport` _marker 0)
  (`/Game/DragonCore/HUD/Widgets/WDG_CompassMarker.InitMarker` _marker (`self.Marker Color`) (`self.Undiscovered`) self)
  (`Widget.SetVisibility` (`self.Marker`) "Collapsed"))

(event `self.DiscoverRange.OnComponentBeginOverlap`
  (params (OverlappedComponent :type "PrimitiveComponent Object Reference") (OtherActor :type "Actor Object Reference") (OtherComp :type "PrimitiveComponent Object Reference") (OtherBodyIndex :type Integer) (bFromSweep :type Boolean) (SweepResult :type "HitResult Structure (by ref)"))
  (bind _returnvalue (`self.GetComponentByClass` OtherActor "/Game/DragonCore/PlayerTabs/WorldMapSystem/Actors/BPC_WorldMap.BPC_WorldMap_C"))
  (bind _marker (`self.Marker`))
  (`|ExecutionSequence`
    (:`then_0`
      (cast `/Game/ThirdPerson/Blueprints/BP_ThirdPersonCharacter` OtherActor)
      (`Widget.RemoveFromParent` (`self.Marker`))
      (`UserWidget.AddToViewport` _marker 0)
      (`/Game/DragonCore/HUD/Widgets/WDG_CompassMarker.InitMarker` _marker (`self.Marker Color`) (`self.TypeOfPOI_Compass`) self))
    (:`then_1`
      (`/Engine/EditorBlueprintResources/StandardMacros.IsValid` _returnvalue
        (:`Is Valid`
          (`/Engine/EditorBlueprintResources/StandardMacros.DoOnce` false
            (:`Completed`
              (`/Game/DragonCore/PlayerTabs/WorldMapSystem/Actors/BPC_WorldMap.OnDiscoveredPointOfInterest` _returnvalue self (`self.TypeOfPOI_Map`)))))))))

(event `OnDiscovered`
  (`ActorComponent.K2_DestroyComponent` (`self.DiscoverRange`))
  (`Widget.SetVisibility` (`self.Marker`) "Visible"))

(event `self.SeeDistance.OnComponentBeginOverlap`
  (params (OverlappedComponent :type "PrimitiveComponent Object Reference") (OtherActor :type "Actor Object Reference") (OtherComp :type "PrimitiveComponent Object Reference") (OtherBodyIndex :type Integer) (bFromSweep :type Boolean) (SweepResult :type "HitResult Structure (by ref)"))
  (cast `/Game/ThirdPerson/Blueprints/BP_ThirdPersonCharacter` OtherActor)
  (`Widget.SetVisibility` (`self.Marker`) "Visible"))

(event `self.SeeDistance.OnComponentEndOverlap`
  (params (OverlappedComponent :type "PrimitiveComponent Object Reference") (OtherActor :type "Actor Object Reference") (OtherComp :type "PrimitiveComponent Object Reference") (OtherBodyIndex :type Integer))
  (cast `/Game/ThirdPerson/Blueprints/BP_ThirdPersonCharacter` OtherActor)
  (`Widget.SetVisibility` (`self.Marker`) "Collapsed"))

(fn `GetMapIconData`
  (returns (Location :type "Vector Structure") (Icon :type "Texture2D Object Reference") (IconSize :type "Vector2D Structure") (`Rotation Yaw` :type "Float (double-precision)") (`World Actor` :type "Actor Object Reference"))
  (return (`self.K2_GetActorLocation`) "/Game/DragonCore/PlayerTabs/WorldMapSystem/Textures/MapIconQuestionMark.MapIconQuestionMark" (30.0 30.0) 0.0 self))

(fn `UserConstructionScript`
  (`SphereComponent.SetSphereRadius` (`self.DiscoverRange`) (`self.DiscoverRadius`) false)
  (`SphereComponent.SetSphereRadius` (`self.SeeDistance`) (`self.SeeRadius`) false))