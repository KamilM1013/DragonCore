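; BP_CustomMarker is a world map actor that represents a custom marker and shows it through a WDG_CompassMarker widget.
; Shortly after BeginPlay it creates the widget and initializes it with the player's chosen color from BPCWorldMap, an exclamation material and itself as owner.
; An OnDestroyed handler, bound from Tick, removes the widget with the actor.
; The Trigger overlap does nothing, as its removal logic is disconnected.
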(event `self.ReceiveBeginPlay`
  (bind _marker (`self.Marker`))
  (bind _asbp_third_person_character (cast `/Game/ThirdPerson/Blueprints/BP_ThirdPersonCharacter` (`GameplayStatics.GetPlayerCharacter` 0)))
  (`KismetSystemLibrary.Delay` 0.2)
  (bind _returnvalue (`|CreateWidget` "/Game/DragonCore/HUD/Widgets/WDG_CompassMarker.WDG_CompassMarker_C"))
  (set `self.Marker` _returnvalue)
  (`UserWidget.AddToViewport` _marker 0)
  (`/Game/DragonCore/HUD/Widgets/WDG_CompassMarker.InitMarker` _marker (`/Game/DragonCore/PlayerTabs/WorldMapSystem/Actors/BPC_WorldMap.ChosenColor` (`/Game/ThirdPerson/Blueprints/BP_ThirdPersonCharacter.BPC_WorldMap` _asbp_third_person_character)) "/Game/DragonCore/HUD/Materials/MInst_ExclamationMarker.MInst_ExclamationMarker" self))

(event `self.ReceiveTick`
  (params (DeltaSeconds :type "Float (single-precision)"))
  (add `self.OnDestroyed` (delegate `OnDestroyed_Event`)))

(event `OnDestroyed_Event` :!signature `self.OnDestroyed`
  (params (DestroyedActor :type "Actor Object Reference"))
  (`Widget.RemoveFromParent` (`self.Marker`)))

(event `self.Trigger.OnComponentBeginOverlap`
  (params (OverlappedComponent :type "PrimitiveComponent Object Reference") (OtherActor :type "Actor Object Reference") (OtherComp :type "PrimitiveComponent Object Reference") (OtherBodyIndex :type Integer) (bFromSweep :type Boolean) (SweepResult :type "HitResult Structure (by ref)")))

(fn `UserConstructionScript`)