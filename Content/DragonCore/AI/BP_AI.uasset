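; Melee enemy AI character with random sword combos, health and ragdoll death.
; A behavior tree entry triggers random montage attacks, with a saved-attack flag chaining combos.
; A looping timer sphere-traces along the weapon, alongside a one-shot trace for stab/kick, damaging "Damageable" actors with shake, sound and blood.
; Taking damage shows a camera-facing health bar, plays hit reactions, launches it along the player's facing and ragdolls on death.
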(event `self.ReceiveBeginPlay`
  (bind _aswb_dummy_health_bar (cast `/Game/DragonCore/UI/WB_DummyHealthBar` (`WidgetComponent.GetWidget` (`self.Health Bar Widget`))))
  (set `self.Health Bar UI` _aswb_dummy_health_bar)
  (`SceneComponent.SetVisibility` (`self.Health Bar Widget`) false false))

(event `self.ReceiveTick`
  (params (DeltaSeconds :type "Float (single-precision)"))
  (bind _health_bar_widget (`self.Health Bar Widget`))
  (`SceneComponent.K2_SetWorldRotation` _health_bar_widget (`KismetMathLibrary.FindLookAtRotation` (`SceneComponent.K2_GetComponentLocation` _health_bar_widget) (`SceneComponent.K2_GetComponentLocation` (`PlayerCameraManager.TransformComponent` (`GameplayStatics.GetPlayerCameraManager` 0)))) false false))

(event `Ragdoll`
  ;[0.05127 0.05127 0.05127] Die
  (`|ExecutionSequence`
    (:`then_0`
      (`GameplayStatics.PlaySoundAtLocation` "/Game/DragonCore/Audio/Grunts/DeathGrunt.DeathGrunt" (`self.K2_GetActorLocation`) (struct) 1.0 1.0 0.0 null null null null))
    (:`then_1`
      (`PrimitiveComponent.SetSimulatePhysics` (`self.Mesh`) true))
    (:`then_2`
      (set `self.isDead` true))))

(event `self.ReceiveAnyDamage`
  (params (Damage :type "Float (single-precision)") (DamageType :type "DamageType Object Reference") (InstigatedBy :type "Controller Object Reference") (DamageCauser :type "Actor Object Reference"))
  (`SceneComponent.SetVisibility` (`self.Health Bar Widget`) true false)
  (`self.PlayAnimMontage` (`|GetArrayItem` (`self.HitAnims`) (`KismetMathLibrary.RandomIntegerInRange` 0 (- (`KismetArrayLibrary.Array_Length` (`self.HitAnims`)) 1))))
  (bind _asbp_third_person_character (cast `/Game/ThirdPerson/Blueprints/BP_ThirdPersonCharacter` (`GameplayStatics.GetPlayerCharacter` 0)))
  (`self.LaunchCharacter` (* (`KismetMathLibrary.GetForwardVector` (`self.K2_GetActorRotation` _asbp_third_person_character)) 700))
  (`GameplayStatics.PlaySoundAtLocation` "/Game/DragonCore/Audio/Grunts/DeathGrunt.DeathGrunt" (`self.K2_GetActorLocation`) (struct) 1.0 (`KismetMathLibrary.RandomFloatInRange` 0.75 1.0) 0.0 "/Game/DragonCore/Audio/SA_Character.SA_Character" null null null)
  (bind _isplayerdead_ (`/Game/DragonCore/Blueprints/BPC_PlayerStats.Decrease Health` (`self.BPC_PlayerStats`) Damage))
  (if _isplayerdead_
    (`PrimitiveComponent.SetCollisionObjectType` (`self.Mesh`) "ECC_PhysicsBody")
    (`self.Ragdoll`)
    (`SceneComponent.SetVisibility` (`self.Health Bar Widget`) false false)
    (`SceneComponent.SetVisibility` (`self.LockOn Widget`) false false)))

(event `Attack 1`
  ;[0.05127 0.05127 0.05127] Combo System
  ;;[0.05127 0.05127 0.05127] Attack 1
  (`/Engine/EditorBlueprintResources/StandardMacros.DoOnce` false :!label _label
    (:`Completed`
      (`KismetSystemLibrary.Delay` 0.1)
      (`|PlayMontage` (`self.Mesh`) "/Game/DragonCore/DragonCharacter/Animations/SwordAttacks/Attack1_Montage.Attack1_Montage"
        (:`then`
          (set `self.AttackIndex` 1)
          (goto _label :!via `Reset`))))))

(event `SwordAttackComboCallFromBT`
  ;[0.05127 0.05127 0.05127] Combo System
  ;;[0.05127 0.05127 0.05127] Attack Event from BT
  (if (`self.canAttack?`)
    (`self.SwordAttack`)))

(event `Attack 2`
  ;[0.05127 0.05127 0.05127] Combo System
  ;;[0.05127 0.05127 0.05127] Attack 2
  (`/Engine/EditorBlueprintResources/StandardMacros.DoOnce` false :!label _label_2
    (:`Completed`
      (`KismetSystemLibrary.Delay` 0.1)
      (`|PlayMontage` (`self.Mesh`) "/Game/DragonCore/DragonCharacter/Animations/SwordAttacks/Attack2_Montage.Attack2_Montage"
        (:`then`
          (set `self.AttackIndex` 2)
          (goto _label_2 :!via `Reset`))))))

(event `SwordAttack`
  ;[0.05127 0.05127 0.05127] Combo System
  ;;[0.05127 0.05127 0.05127] Sword Attack
  (if (`self.isAttacking?`)
    (set `self.saveAttack?` true)
    (else
      (set `self.isAttacking?` true)
      (switch `int` (`KismetMathLibrary.RandomIntegerInRange` 0 2) :!label _label_3
        (:`0`
          (`self.Attack 1`))
        (:`1`
          (`self.Attack 2`))
        (:`2`
          (`self.Attack 4`))))))

(event `Attack 3`
  ;[0.05127 0.05127 0.05127] Combo System
  ;;[0.05127 0.05127 0.05127] Attack 3/Not using at the moment
  (`/Engine/EditorBlueprintResources/StandardMacros.DoOnce` false :!label _label_4
    (:`Completed`
      (`KismetSystemLibrary.Delay` 0.1)
      (`|PlayMontage` (`self.Mesh`) "/Game/DragonCore/DragonCharacter/Animations/SwordAttacks/Kick_Montage.Kick_Montage"
        (:`then`
          (set `self.AttackIndex` 3)
          (goto _label_4 :!via `Reset`))))))

(event `SwordAttackCombo`
  ;[0.05127 0.05127 0.05127] Combo System
  ;;[0.05127 0.05127 0.05127] Combo Continue
  (if (`self.saveAttack?`)
    (set `self.saveAttack?` false)
    (goto _label_3)
    (else
      (`self.StopCombo`))))

(event `StopCombo`
  ;[0.05127 0.05127 0.05127] Combo System
  ;;[0.05127 0.05127 0.05127] Stop Combo
  (set `self.isAttacking?` false)
  (set `self.AttackIndex` 0))

(event `Attack 4`
  ;[0.05127 0.05127 0.05127] Combo System
  ;;[0.05127 0.05127 0.05127] Attack 4
  (`/Engine/EditorBlueprintResources/StandardMacros.DoOnce` false :!label _label_5
    (:`Completed`
      (`KismetSystemLibrary.Delay` 0.1)
      (`|PlayMontage` (`self.Mesh`) "/Game/DragonCore/DragonCharacter/Animations/SwordAttacks/Attack3_Montage.Attack3_Montage"
        (:`then`
          (set `self.AttackIndex` 4)
          (goto _label_5 :!via `Reset`))))))

(event `StartAttackTrace`
  ;[0.05127 0.05127 0.05127] Sword Trace
  (bind _returnvalue (`KismetSystemLibrary.K2_SetTimerDelegate` (delegate `AttackTraceLoop`) 0.001 true))
  (set `self.AttackTrace` _returnvalue))

(event `AttackTraceLoop`
  ;[0.05127 0.05127 0.05127] Sword Trace
  (bind (_outhit _returnvalue) (`KismetSystemLibrary.SphereTraceSingle` :`Start` (`SceneComponent.K2_GetComponentLocation` (`self.WeaponTopPoint`)) :`End` (`SceneComponent.K2_GetComponentLocation` (`self.WeaponBottomPoint`)) :`Radius` 12.0 :`TraceChannel` "TraceTypeQuery1" :`DrawTime` 0.2))
  (if _returnvalue
    (bind (_bblockinghit _binitialoverlap _time _distance _location _impactpoint _normal _impactnormal _physmat _hitactor) (`GameplayStatics.BreakHitResult` _outhit))
    (if (`self.ActorHasTag` _hitactor "Damageable")
      (`/Engine/EditorBlueprintResources/StandardMacros.DoOnce` false :!label _label_6
        (:`Completed`
          (`GameplayStatics.ApplyDamage` _hitactor 10.0)
          (`GameplayStatics.PlayWorldCameraShake` "/Game/DragonCore/Blueprints/BP_HitCameraShake.BP_HitCameraShake_C" _location 0.0 2000.0)
          (`self.PlayAttackHitSounds`)
          (`GameplayStatics.SpawnEmitterAtLocation` "/Game/Realistic_Starter_VFX_Pack_Vol2/Particles/Blood/P_Blood_Splat_Cone.P_Blood_Splat_Cone" _location (`KismetMathLibrary.MakeRotFromXY` _normal _normal) (0.4 0.4 0.4) true "AutoRelease")
          (`KismetSystemLibrary.Delay` 0.5)
          (goto _label_6 :!via `Reset`))))))

(event `StopAttackTrace`
  ;[0.05127 0.05127 0.05127] Sword Trace
  (`KismetSystemLibrary.K2_ClearAndInvalidateTimerHandle` (`self.AttackTrace`)))

(event `PlayAttackHitSounds`
  ;[0.05127 0.05127 0.05127] Play Attack Hit Sounds
  (`GameplayStatics.PlaySoundAtLocation` "/Game/DragonCore/Audio/Hits/MS_AttackHits.MS_AttackHits" (`self.K2_GetActorLocation` (`self.GetOwner`)) (struct) 1.0 1.0 0.0 null null null null))

(event `SphereTrace`
  (bind _returnvalue (`SceneComponent.K2_GetComponentLocation` (`self.SphereTracePos`)))
  ;[0.05127 0.05127 0.05127] Sphere Trace (Stab/Kick)
  (bind (_outhit _returnvalue_2) (`KismetSystemLibrary.SphereTraceSingle` :`Start` _returnvalue :`End` _returnvalue :`Radius` 25.0 :`TraceChannel` "TraceTypeQuery1" :`DrawTime` 0.2))
  (if _returnvalue_2
    (bind (_bblockinghit _binitialoverlap _time _distance _location _impactpoint _normal _impactnormal _physmat _hitactor) (`GameplayStatics.BreakHitResult` _outhit))
    (if (`self.ActorHasTag` _hitactor "Damageable")
      (`GameplayStatics.ApplyDamage` _hitactor 10.0)
      (`GameplayStatics.PlayWorldCameraShake` "/Game/DragonCore/Blueprints/BP_HitCameraShake.BP_HitCameraShake_C" _location 0.0 2000.0)
      (`self.PlayAttackHitSounds`)
      (`GameplayStatics.SpawnEmitterAtLocation` "/Game/Realistic_Starter_VFX_Pack_Vol2/Particles/Blood/P_Blood_Splat_Cone.P_Blood_Splat_Cone" _location (`KismetMathLibrary.MakeRotFromXY` _normal _normal) (0.4 0.4 0.4) true "AutoRelease"))))

(fn `Attack`
  (returns (AnimationDuration :type "Float (double-precision)"))
  (`self.SwordAttackComboCallFromBT`)
  (return 0.4))

(fn `Run`
  (returns (`isRunning?` :type Boolean))
  (set `CharacterMovementComponent.MaxWalkSpeed` 450.0 (`self.CharacterMovement`))
  (return true))

(fn `UserConstructionScript`)

(fn `Walk`
  (returns (`isWalking?` :type Boolean))
  (set `CharacterMovementComponent.MaxWalkSpeed` 250.0 (`self.CharacterMovement`))
  (return true))