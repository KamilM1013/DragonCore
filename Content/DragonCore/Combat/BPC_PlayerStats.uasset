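; Stats component for the player and Master_Enemy actors that tracks health, plus rage, XP and level for the player.
; Stat functions update the matching HUD or enemy bars directly, with decrease calls returning whether the stat is depleted.
; Tick lerps a back health bar toward current health for a trailing damage effect.
; XP overflow loops through level-ups, scaling max XP and health and triggering sounds, aura and HUD fade; mana is deprecated.
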(event `InitPlayerStats`
  (params (PlayerCharacter :type "/Game/ThirdPerson/Blueprints/BP_ThirdPersonCharacter Object Reference"))
  ;[0.05127 0.05127 0.05127] Initialize player character references
  (bind _output_get (set `self.PlayerCharacter` PlayerCharacter))
  (set `self.NS Aura` (`/Game/ThirdPerson/Blueprints/BP_ThirdPersonCharacter.NS_Aura` _output_get))
  (set `self.HUD Level` (`/Game/ThirdPerson/Blueprints/BP_ThirdPersonCharacter.HUD Level` _output_get)))

(event `self.ReceiveBeginPlay`
  ;[0.05127 0.05127 0.05127] Initializing all Progress Bars
  (`KismetSystemLibrary.DelayUntilNextTick`)
  (bind _asmaster_enemy (cast `/Game/DragonCore/AI_Classes/Enemies/Master_Enemy` (`self.GetOwner`))
    (:`then`
      (set `self.MasterEnemy` _asmaster_enemy)
      (set `self.isPlayer` false))
    (:`CastFailed`
      (set `self.isPlayer` true)
      (`ProgressBar.SetPercent` (`/Game/DragonCore/HUD/Widgets/WB_HUD.RageBar` (`/Game/ThirdPerson/Blueprints/BP_ThirdPersonCharacter.HUD_Widget` (`self.PlayerCharacter`))) (`KismetMathLibrary.MapRangeClamped` (`self.Current Rage`) 0.0 (`self.Max Rage`) 0.0 1.0))
      (`ProgressBar.SetPercent` (`/Game/DragonCore/HUD/Widgets/WB_Level.XPBar` (`/Game/ThirdPerson/Blueprints/BP_ThirdPersonCharacter.HUD Level` (`self.PlayerCharacter`))) (`KismetMathLibrary.MapRangeClamped` (`self.XP`) 0.0 (`self.Max XP`) 0.0 1.0))
      (`TextBlock.SetText` (`/Game/DragonCore/HUD/Widgets/WB_Level.Level` (`/Game/ThirdPerson/Blueprints/BP_ThirdPersonCharacter.HUD Level` (`self.PlayerCharacter`))) (`KismetTextLibrary.Conv_IntToText` (`self.Level`)))))
  (`ProgressBar.SetPercent` (select `bool` (`self.isPlayer`) :`false` (`/Game/DragonCore/HUD/Widgets/WB_EnemyHealthBar.HealthBar` (`/Game/DragonCore/AI_Classes/Enemies/Master_Enemy.HealthBar Ref` (`self.MasterEnemy`))) :`true` (`/Game/DragonCore/HUD/Widgets/WB_HUD.HealthBar` (`/Game/ThirdPerson/Blueprints/BP_ThirdPersonCharacter.HUD_Widget` (`self.PlayerCharacter`)))) (`KismetMathLibrary.MapRangeClamped` (`self.Current Health`) 0.0 (`self.Max Health`) 0.0 1.0)))

(event `self.ReceiveTick`
  (params (DeltaSeconds :type "Float (single-precision)"))
  (bind _healthbarback (`/Game/DragonCore/HUD/Widgets/WB_HUD.HealthBarBack` (`/Game/ThirdPerson/Blueprints/BP_ThirdPersonCharacter.HUD_Widget` (`self.PlayerCharacter`))))
  ;[0.05127 0.05127 0.05127] Adds effect to Health Bar while decreasing health
  (bind _asmaster_enemy (cast `/Game/DragonCore/AI_Classes/Enemies/Master_Enemy` (`self.GetOwner`))
    (:`then`
      (bind _healthbarback_2 (`/Game/DragonCore/HUD/Widgets/WB_EnemyHealthBar.HealthBarBack` (`/Game/DragonCore/AI_Classes/Enemies/Master_Enemy.HealthBar Ref` _asmaster_enemy)))
      (`ProgressBar.SetPercent` _healthbarback_2 (`KismetMathLibrary.Lerp` (`ProgressBar.Percent` _healthbarback_2) (/ (`self.Current Health`) (`self.Max Health`)) 0.05)))
    (:`CastFailed`
      (`ProgressBar.SetPercent` _healthbarback (`KismetMathLibrary.Lerp` (`ProgressBar.Percent` _healthbarback) (/ (`self.Current Health`) (`self.Max Health`)) 0.05)))))

(event `LevelUp`
  (bind _ns_aura (`self.NS Aura`))
  (bind _hud_level (`self.HUD Level`))
  (bind _fadein (`/Game/DragonCore/HUD/Widgets/WB_Level.FadeIn` _hud_level))
  ;[0.05127 0.05127 0.05127] Level up
  (`|ExecutionSequence`
    (:`then_0`
      (`self.Activate` _ns_aura false)
      (`KismetSystemLibrary.Delay` 1.0)
      (`self.Deactivate` _ns_aura))
    (:`then_1`
      (`UserWidget.AddToViewport` _hud_level 0)
      (`UserWidget.PlayAnimation` _hud_level _fadein 0.0 1 "Forward" 1.0 false)
      (`KismetSystemLibrary.Delay` 3.0)
      (`UserWidget.PlayAnimation` _hud_level _fadein 0.0 1 "Reverse" 1.0 false)
      (`KismetSystemLibrary.Delay` 0.5)
      (`Widget.RemoveFromParent` _hud_level))))

(fn `Decrease Health`
  (params (Damage :type "Float (double-precision)"))
  (returns (`isPlayerDead?` :type Boolean))
  (if (not (<= (`self.Current Health`) 0.0))
    (bind _output_get (set `self.Current Health` (- (`self.Current Health`) Damage)))
    (`ProgressBar.SetPercent` (select `bool` (`self.isPlayer`) :`false` (`/Game/DragonCore/HUD/Widgets/WB_EnemyHealthBar.HealthBar` (`/Game/DragonCore/AI_Classes/Enemies/Master_Enemy.HealthBar Ref` (`self.MasterEnemy`))) :`true` (`/Game/DragonCore/HUD/Widgets/WB_HUD.HealthBar` (`/Game/ThirdPerson/Blueprints/BP_ThirdPersonCharacter.HUD_Widget` (`self.PlayerCharacter`)))) (`KismetMathLibrary.MapRangeClamped` _output_get 0.0 (`self.Max Health`) 0.0 1.0))
    (if (<= (`self.Current Health`) 0.0)
      _
      (else
        (return false))))
  (return true))

(fn `Decrease Mana`
  (params (`Mana Depleted` :type "Float (double-precision)"))
  (returns (`No Mana` :type Boolean))
  ;[1 0.03692 0] Deprecated
)

(fn `Decrease Rage`
  (params (`Rage Depleted` :type "Float (double-precision)"))
  (returns (`No Rage` :type Boolean))
  (if (not (<= (`self.Current Rage`) 0.0))
    (bind _output_get (set `self.Current Rage` (- (`self.Current Rage`) `Rage Depleted`)))
    (`ProgressBar.SetPercent` (`/Game/DragonCore/HUD/Widgets/WB_HUD.RageBar` (`/Game/ThirdPerson/Blueprints/BP_ThirdPersonCharacter.HUD_Widget` (`self.PlayerCharacter`))) (`KismetMathLibrary.MapRangeClamped` _output_get 0.0 (`self.Max Rage`) 0.0 1.0))
    (if (<= (`self.Current Rage`) 0.0)
      _
      (else
        (return false))))
  (return true))

(fn `Increase Health`
  (params (`Added Health` :type "Float (double-precision)"))
  (bind _max_health (`self.Max Health`))
  (bind _healthbar (`/Game/DragonCore/HUD/Widgets/WB_HUD.HealthBar` (`/Game/ThirdPerson/Blueprints/BP_ThirdPersonCharacter.HUD_Widget` (`self.PlayerCharacter`))))
  (bind _output_get (set `self.Current Health` (+ (`self.Current Health`) `Added Health`)))
  (if (> _output_get (`self.Max Health`))
    (bind _output_get_2 (set `self.Current Health` _max_health))
    (`ProgressBar.SetPercent` _healthbar (`KismetMathLibrary.MapRangeClamped` _output_get_2 0.0 _max_health 0.0 1.0))
    (else
      (`ProgressBar.SetPercent` _healthbar (`KismetMathLibrary.MapRangeClamped` _output_get 0.0 _max_health 0.0 1.0)))))

(fn `Increase Level`
  (params (`Added Level` :type Integer))
  (set `self.Level` (+ (`self.Level`) `Added Level`))
  (set `self.XP` (- (`self.XP`) (`self.Max XP`)))
  (set `self.Max XP` (`KismetMathLibrary.Conv_IntToDouble` (`KismetMathLibrary.FFloor` (* (`self.Max XP`) 1.5))))
  (set `self.Max Health` (`KismetMathLibrary.Conv_IntToDouble` (`KismetMathLibrary.FFloor` (* (`self.Max Health`) 1.2))))
  (`TextBlock.SetText` (`/Game/DragonCore/HUD/Widgets/WB_Level.Level` (`/Game/ThirdPerson/Blueprints/BP_ThirdPersonCharacter.HUD Level` (`self.PlayerCharacter`))) (`KismetTextLibrary.Conv_IntToText` (`self.Level`)))
  (`GameplayStatics.PlaySound2D` "/Game/DragonCore/Audio/UI/LevelUp.LevelUp" 1.0 1.0 0.0 null null)
  (`GameplayStatics.PlaySound2D` "/Game/DragonCore/Audio/UI/LevelUp2.LevelUp2" 1.0 1.0 0.0 null null)
  (`self.LevelUp`))

(fn `Increase Mana`
  (params (`Added Mana` :type "Float (double-precision)"))
  ;[1 0.03692 0] Deprecated
)

(fn `Increase Max Health`
  (params (`Added Health` :type "Float (double-precision)"))
  (bind _output_get (set `self.Max Health` (+ (`self.Max Health`) `Added Health`)))
  (`ProgressBar.SetPercent` (select `bool` (`self.isPlayer`) :`false` (`/Game/DragonCore/HUD/Widgets/WB_EnemyHealthBar.HealthBar` (`/Game/DragonCore/AI_Classes/Enemies/Master_Enemy.HealthBar Ref` (`self.MasterEnemy`))) :`true` (`/Game/DragonCore/HUD/Widgets/WB_HUD.HealthBar` (`/Game/ThirdPerson/Blueprints/BP_ThirdPersonCharacter.HUD_Widget` (`self.PlayerCharacter`)))) (`KismetMathLibrary.FClamp` _output_get)))

(fn `Increase Max Mana`
  (params (`Added Mana` :type "Float (double-precision)"))
  ;[1 0.03692 0] Deprecated
)

(fn `Increase Rage`
  (params (`Added Rage` :type "Float (double-precision)"))
  (bind _max_rage (`self.Max Rage`))
  (bind _ragebar (`/Game/DragonCore/HUD/Widgets/WB_HUD.RageBar` (`/Game/ThirdPerson/Blueprints/BP_ThirdPersonCharacter.HUD_Widget` (`self.PlayerCharacter`))))
  (bind _output_get (set `self.Current Rage` (+ (`self.Current Rage`) `Added Rage`)))
  (if (> _output_get (`self.Max Rage`))
    (bind _output_get_2 (set `self.Current Rage` _max_rage))
    (`ProgressBar.SetPercent` _ragebar (`KismetMathLibrary.MapRangeClamped` _output_get_2 0.0 _max_rage 0.0 1.0))
    (else
      (`ProgressBar.SetPercent` _ragebar (`KismetMathLibrary.MapRangeClamped` _output_get 0.0 _max_rage 0.0 1.0)))))

(fn `Increase XP`
  (params (`Added XP` :type "Float (double-precision)"))
  (bind _output_get (set `self.XP` (+ (`self.XP`) `Added XP`)))
  (while (>= _output_get (`self.Max XP`))
    (`self.Increase Level` 1)
    (`ProgressBar.SetPercent` (`/Game/DragonCore/HUD/Widgets/WB_Level.XPBar` (`/Game/ThirdPerson/Blueprints/BP_ThirdPersonCharacter.HUD Level` (`self.PlayerCharacter`))) (`KismetMathLibrary.MapRangeClamped` (`self.XP`) 0.0 (`self.Max XP`) 0.0 1.0) :!label _label))
  (goto _label))