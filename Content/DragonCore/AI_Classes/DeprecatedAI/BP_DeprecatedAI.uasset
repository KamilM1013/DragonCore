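; Deprecated sword-wielding enemy character that spots, fights and chases the player, or returns to its spawn post.
; PawnSensing drives an AIMoveTo state loop in the event graph, randomly choosing between strafing and closing in for a random montage attack.
; Timer-looped sphere traces along the weapon deal damage, with Damage and XP scaled by level.
; Hits trigger knockback and a health bar; death ragdolls it, granting XP only if the player is locked on.
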(event `self.ReceiveBeginPlay`
  ;[0.05127 0.05127 0.05127] Setup
  (bind _aswb_dummy_health_bar (cast `/Game/DragonCore/UI_HUD/WB_DummyHealthBar` (`WidgetComponent.GetWidget` (`self.Health Bar Widget`))))
  (set `self.Health Bar UI` _aswb_dummy_health_bar)
  (`SceneComponent.SetVisibility` (`self.Health Bar Widget`) false false)
  (set `self.EnemyPost` (`self.K2_GetActorLocation`))
  (`self.SetStatsByLevel`))

(event `self.ReceiveTick`
  (params (DeltaSeconds :type "Float (single-precision)"))
  (bind _target (`self.Target`))
  (bind _health_bar_widget (`self.Health Bar Widget`))
  ;[0.05127 0.05127 0.05127] Rotate to Player
  (`|ExecutionSequence`
    (:`then_0`
      ;;[0.05127 0.05127 0.05127] Rotate Enemy to Player
      (if (`self.hasTarget?`)
        (`/Engine/EditorBlueprintResources/StandardMacros.IsValid` _target
          (:`Is Valid`
            (if (`self.isStrafing?`)
              (set `self.ActorRotation` (`self.K2_GetActorRotation`))
              (bind (_direction _length) (`Timeline|Timeline`)
                (:`Update`
                  (`self.K2_SetActorRotation` (`KismetMathLibrary.RLerp` (`self.ActorRotation`) (`KismetMathLibrary.FindLookAtRotation` (`self.K2_GetActorLocation`) (`self.K2_GetActorLocation` _target)) _length))
                  ;;[0.05127 0.05127 0.05127] Set Strafing Direction
                  (`self.AddMovementInput` (`self.SetStrafingDirection`)))))))))
    (:`then_1`
      ;;[0.05127 0.05127 0.05127] Rotate Hud to Player
      (if (and (not (`self.isDead`)) (`self.hasTarget?`))
        (`SceneComponent.K2_SetWorldRotation` _health_bar_widget (`KismetMathLibrary.FindLookAtRotation` (`SceneComponent.K2_GetComponentLocation` _health_bar_widget) (`SceneComponent.K2_GetComponentLocation` (`PlayerCameraManager.TransformComponent` (`GameplayStatics.GetPlayerCameraManager` 0)))) false false)))))

(event `Death`
  (bind _sword (`self.Sword`))
  (bind _sword_2 (`self.Sword`))
  ;[0.05127 0.05127 0.05127] Die
  (set `self.canAttack?` false)
  (set `self.isDead` true)
  (`self.Hide HealthBar`)
  (`SceneComponent.SetVisibility` (`self.LockOn Widget`) false false)
  (`GameplayStatics.PlaySoundAtLocation` "/Game/DragonCore/Audio/Grunts/DeathGrunt.DeathGrunt" (`self.K2_GetActorLocation`) (struct) 1.0 1.0 0.0 null null null null)
  (`PrimitiveComponent.SetSimulatePhysics` (`self.Mesh`) true)
  (`SceneComponent.K2_DetachFromComponent` _sword_2 "KeepWorld" "KeepWorld" "KeepWorld" true)
  (`PrimitiveComponent.SetCollisionEnabled` _sword_2 "QueryAndPhysics")
  (`PrimitiveComponent.SetSimulatePhysics` _sword true)
  (`PrimitiveComponent.SetCollisionObjectType` _sword "ECC_WorldStatic")
  (`PrimitiveComponent.SetCollisionObjectType` (`self.Mesh`) "ECC_WorldStatic")
  (bind _asbp_third_person_character (cast `/Game/ThirdPerson/Blueprints/BP_ThirdPersonCharacter` (`GameplayStatics.GetPlayerCharacter` 0)))
  (if (`/Game/ThirdPerson/Blueprints/BP_ThirdPersonCharacter.isLocked?` _asbp_third_person_character)
    (`/Game/ThirdPerson/Blueprints/BP_ThirdPersonCharacter.Lock/Unlock` _asbp_third_person_character)
    (bind _asbp_third_person_character_2 (cast `/Game/ThirdPerson/Blueprints/BP_ThirdPersonCharacter` (`GameplayStatics.GetPlayerCharacter` 0)))
    (`/Game/DragonCore/Blueprints/BPC_PlayerStats.Increase XP` (`/Game/ThirdPerson/Blueprints/BP_ThirdPersonCharacter.BPC_PlayerStats` _asbp_third_person_character_2) (`self.XP`)))
  (`KismetSystemLibrary.Delay` 30.0)
  (`self.K2_DestroyActor`))

(event `self.ReceiveAnyDamage`
  (params (Damage :type "Float (single-precision)") (DamageType :type "DamageType Object Reference") (InstigatedBy :type "Controller Object Reference") (DamageCauser :type "Actor Object Reference"))
  ;[0.05127 0.05127 0.05127] Taking Damage
  (`/Engine/EditorBlueprintResources/StandardMacros.DoOnce` false :!label _label
    (:`Completed`
      (`|ExecutionSequence`
        (:`then_0`
          (set `self.mustAttack?` true)
          (`self.Show HealthBar`)
          (`self.PlayAnimMontage` (`|GetArrayItem` (`self.HitAnims`) (`KismetMathLibrary.RandomIntegerInRange` 0 (- (`KismetArrayLibrary.Array_Length` (`self.HitAnims`)) 1))))
          (bind _asbp_third_person_character (cast `/Game/ThirdPerson/Blueprints/BP_ThirdPersonCharacter` (`GameplayStatics.GetPlayerCharacter` 0)))
          (`self.LaunchCharacter` (* (`KismetMathLibrary.GetForwardVector` (`self.K2_GetActorRotation` _asbp_third_person_character)) 700))
          (`GameplayStatics.PlaySoundAtLocation` "/Game/DragonCore/Audio/Grunts/DeathGrunt.DeathGrunt" (`self.K2_GetActorLocation`) (struct) 1.0 (`KismetMathLibrary.RandomFloatInRange` 0.75 1.0) 0.0 "/Game/DragonCore/Audio/SA_Character.SA_Character" null null null)
          (bind _isplayerdead_ (`/Game/DragonCore/Blueprints/BPC_PlayerStats.Decrease Health` (`self.BPC_PlayerStats`) Damage))
          (if _isplayerdead_
            (`self.Death`)))
        (:`then_1`
          (`KismetSystemLibrary.Delay` 0.5)
          (goto _label :!via `Reset`))))))

(event `Attack 1`
  ;[0.05127 0.05127 0.05127] Combo System
  ;;[0.05127 0.05127 0.05127] Attack 1
  (`/Engine/EditorBlueprintResources/StandardMacros.DoOnce` false :!label _label_2
    (:`Completed`
      (`KismetSystemLibrary.Delay` 0.1)
      (`|PlayMontage` (`self.Mesh`) "/Game/DragonCore/DragonCharacter/Animations/SwordAttacks/Attack1_Montage.Attack1_Montage"
        (:`then`
          (set `self.AttackIndex` 1)
          (goto _label_2 :!via `Reset`))))))

(event `SwordAttackComboCallFromBT`
  ;[0.05127 0.05127 0.05127] Combo System
  ;;[0.05127 0.05127 0.05127] Attack Event from BT
  (if (`self.canAttack?`)
    (`self.SwordAttack`)))

(event `Attack 2`
  ;[0.05127 0.05127 0.05127] Combo System
  ;;[0.05127 0.05127 0.05127] Attack 2
  (`/Engine/EditorBlueprintResources/StandardMacros.DoOnce` false :!label _label_3
    (:`Completed`
      (`KismetSystemLibrary.Delay` 0.1)
      (`|PlayMontage` (`self.Mesh`) "/Game/DragonCore/DragonCharacter/Animations/SwordAttacks/Attack2_Montage.Attack2_Montage"
        (:`then`
          (set `self.AttackIndex` 2)
          (goto _label_3 :!via `Reset`))))))

(event `SwordAttack`
  ;[0.05127 0.05127 0.05127] Combo System
  ;;[0.05127 0.05127 0.05127] Sword Attack
  (switch `int` (`KismetMathLibrary.RandomIntegerInRange` 0 2) :!label _label_4
    (:`0`
      (`self.Attack 1`))
    (:`1`
      (`self.Attack 2`))
    (:`2`
      (`self.Attack 4`))))

(event `Attack 3`
  ;[0.05127 0.05127 0.05127] Combo System
  ;;[0.05127 0.05127 0.05127] Attack 3/Not using at the moment
  (`/Engine/EditorBlueprintResources/StandardMacros.DoOnce` false :!label _label_5
    (:`Completed`
      (`KismetSystemLibrary.Delay` 0.1)
      (`|PlayMontage` (`self.Mesh`) "/Game/DragonCore/DragonCharacter/Animations/SwordAttacks/Kick_Montage.Kick_Montage"
        (:`then`
          (set `self.AttackIndex` 3)
          (goto _label_5 :!via `Reset`))))))

(event `SwordAttackCombo`
  ;[0.05127 0.05127 0.05127] Combo System
  ;;[0.05127 0.05127 0.05127] Combo Continue
  (if (`self.saveAttack?`)
    (set `self.saveAttack?` false)
    (goto _label_4)
    (else
      (`self.StopCombo`))))

(event `StopCombo`
  ;[0.05127 0.05127 0.05127] Combo System
  ;;[0.05127 0.05127 0.05127] Stop Combo
  (set `self.isAttacking?` false)
  (set `self.AttackIndex` 0))

(event `Attack 4`
  ;[0.05127 0.05127 0.05127] Combo System
  ;;[0.05127 0.05127 0.05127] Attack 4
  (`/Engine/EditorBlueprintResources/StandardMacros.DoOnce` false :!label _label_6
    (:`Completed`
      (`KismetSystemLibrary.Delay` 0.1)
      (`|PlayMontage` (`self.Mesh`) "/Game/DragonCore/DragonCharacter/Animations/SwordAttacks/Attack3_Montage.Attack3_Montage"
        (:`then`
          (set `self.AttackIndex` 4)
          (goto _label_6 :!via `Reset`))))))

(event `StartAttackTrace`
  ;[0.05127 0.05127 0.05127] Sword Trace
  (bind _returnvalue (`KismetSystemLibrary.K2_SetTimerDelegate` (delegate `AttackTraceLoop`) 0.001 true))
  (set `self.AttackTrace` _returnvalue))

(event `AttackTraceLoop`
  ;[0.05127 0.05127 0.05127] Sword Trace
  (bind (_outhit _returnvalue) (`KismetSystemLibrary.SphereTraceSingle` :`Start` (`SceneComponent.K2_GetComponentLocation` (`self.WeaponTopPoint`)) :`End` (`SceneComponent.K2_GetComponentLocation` (`self.WeaponBottomPoint`)) :`Radius` 12.0 :`TraceChannel` "TraceTypeQuery1" :`DrawDebugType` "ForDuration" :`DrawTime` 0.2))
  (if _returnvalue
    (bind (_bblockinghit _binitialoverlap _time _distance _location _impactpoint _normal _impactnormal _physmat _hitactor) (`GameplayStatics.BreakHitResult` _outhit))
    (if (`self.ActorHasTag` _hitactor "Player")
      (`/Engine/EditorBlueprintResources/StandardMacros.DoOnce` false :!label _label_7
        (:`Completed`
          (if (== (`self.AttackIndex`) 1)
            (`GameplayStatics.ApplyDamage` _hitactor (`self.Damage`))
            (else
              (`GameplayStatics.ApplyDamage` _hitactor (+ (`self.Damage`) 10.0))))
          (`GameplayStatics.PlayWorldCameraShake` "/Game/DragonCore/Blueprints/BP_HitCameraShake.BP_HitCameraShake_C" _location 0.0 2000.0)
          (`self.PlayAttackHitSounds`)
          (`GameplayStatics.SpawnEmitterAtLocation` "/Game/Realistic_Starter_VFX_Pack_Vol2/Particles/Blood/P_Blood_Splat_Cone.P_Blood_Splat_Cone" _location (`KismetMathLibrary.MakeRotFromXY` _normal _normal) (0.4 0.4 0.4) true "AutoRelease")
          (`KismetSystemLibrary.Delay` 0.5)
          (goto _label_7 :!via `Reset`))))))

(event `StopAttackTrace`
  ;[0.05127 0.05127 0.05127] Sword Trace
  (`KismetSystemLibrary.K2_ClearAndInvalidateTimerHandle` (`self.AttackTrace`)))

(event `PlayAttackHitSounds`
  ;[0.05127 0.05127 0.05127] Play Attack Hit Sounds
  (`GameplayStatics.PlaySoundAtLocation` "/Game/DragonCore/Audio/Hits/MS_AttackHits.MS_AttackHits" (`self.K2_GetActorLocation` (`self.GetOwner`)) (struct) 1.0 1.0 0.0 null null null null))

(event `Reset HealthBar`
  ;[0.05127 0.05127 0.05127] Turn On/Off Health Bar
  (`self.Hide HealthBar`))

(event `Show HealthBar`
  ;[0.05127 0.05127 0.05127] Turn On/Off Health Bar
  (`/Engine/EditorBlueprintResources/StandardMacros.IsValid` self
    (:`Is Valid`
      (`SceneComponent.SetVisibility` (`self.Health Bar Widget`) true false)
      (`KismetSystemLibrary.K2_SetTimerDelegate` (delegate `Reset HealthBar`) 20.0))))

(event `_CombatMode?`
  (params (`CombatMode?` :type Boolean) (bOrientRotationToMovement :type Boolean) (bUseControllerDesiredRotation :type Boolean) (MaxWalkSpeed :type "Float (double-precision)"))
  (bind _charactermovement (`self.CharacterMovement`))
  ;[0.05127 0.05127 0.05127] Setup basic variables for combat mode
  (set `self.CombatMode?` `CombatMode?`)
  (set `CharacterMovementComponent.bOrientRotationToMovement` bOrientRotationToMovement _charactermovement)
  (set `CharacterMovementComponent.bUseControllerDesiredRotation` bUseControllerDesiredRotation _charactermovement)
  (set `CharacterMovementComponent.MaxWalkSpeed` MaxWalkSpeed _charactermovement)
  (`KismetSystemLibrary.Delay` 0.3))

(event `Hide HealthBar`
  ;[0.05127 0.05127 0.05127] Turn On/Off Health Bar
  (`/Engine/EditorBlueprintResources/StandardMacros.IsValid` self
    (:`Is Valid`
      (`SceneComponent.SetVisibility` (`self.Health Bar Widget`) false false))))

(event `SphereTrace`
  (bind _returnvalue (`SceneComponent.K2_GetComponentLocation` (`self.SphereTracePos`)))
  ;[0.05127 0.05127 0.05127] Sphere Trace (Stab/Kick)
  (bind (_outhit _returnvalue_2) (`KismetSystemLibrary.SphereTraceSingle` :`Start` _returnvalue :`End` _returnvalue :`Radius` 25.0 :`TraceChannel` "TraceTypeQuery1" :`DrawDebugType` "ForDuration" :`DrawTime` 0.2))
  (if _returnvalue_2
    (bind (_bblockinghit _binitialoverlap _time _distance _location _impactpoint _normal _impactnormal _physmat _hitactor) (`GameplayStatics.BreakHitResult` _outhit))
    (if (`self.ActorHasTag` _hitactor "Player")
      (`GameplayStatics.ApplyDamage` _hitactor (+ (`self.Damage`) 2.0))
      (`GameplayStatics.PlayWorldCameraShake` "/Game/DragonCore/Blueprints/BP_HitCameraShake.BP_HitCameraShake_C" _location 0.0 2000.0)
      (`self.PlayAttackHitSounds`)
      (`GameplayStatics.SpawnEmitterAtLocation` "/Game/Realistic_Starter_VFX_Pack_Vol2/Particles/Blood/P_Blood_Splat_Cone.P_Blood_Splat_Cone" _location (`KismetMathLibrary.MakeRotFromXY` _normal _normal) (0.4 0.4 0.4) true "AutoRelease"))))

(event `self.PawnSensing.OnSeePawn`
  (params (Pawn :type "Pawn Object Reference"))
  ;[0.05127 0.05127 0.05127] Check if AI sees player
  (bind _asbp_third_person_character (cast `/Game/ThirdPerson/Blueprints/BP_ThirdPersonCharacter` Pawn))
  (set `self.Target` _asbp_third_person_character)
  (set `self.seeEnemy?` true)
  (`|ExecutionSequence`
    (:`then_0`
      (`self.SeenTarget`)
      (bind _asbp_third_person_character_2 (cast `/Game/ThirdPerson/Blueprints/BP_ThirdPersonCharacter` (`GameplayStatics.GetPlayerCharacter` 0)))
      (`UserWidget.AddToViewport` (`/Game/ThirdPerson/Blueprints/BP_ThirdPersonCharacter.HUD_Widget` _asbp_third_person_character_2) 0))
    (:`then_1`
      (`KismetSystemLibrary.RetriggerableDelay` 0.6)
      (set `self.seeEnemy?` false)
      (`self.ResetSense`))))

(event `SeenTarget`
  (bind _target (`self.Target`))
  ;[0.05127 0.05127 0.05127] Check if player has been seen
  (`/Engine/EditorBlueprintResources/StandardMacros.DoOnce` false :!label _label
    (:`Completed`
      (if (`self.seeEnemy?`)
        ;[0.05127 0.05127 0.05127] AI goes through this tree when it sees the player
        (set `self.hasTarget?` true)
        (`self.Show HealthBar`)
        (`|AIMoveTo` self (`SceneComponent.K2_GetComponentLocation` (`Character.Mesh` (`self.Target`))) (`self.Target`) 450.0 :!label _label_2
          (:`OnSuccess`
            (if (not (`self.CombatMode?`))
              (`self._CombatMode?` true false true 250.0))
            (if (`self.mustAttack?`)
              (`|AIMoveTo` self (`SceneComponent.K2_GetComponentLocation` (`Character.Mesh` _target)) _target 150.0 :!label _label_3
                (:`OnSuccess`
                  (set `self.isStrafing?` false)
                  (if (not (`/Game/ThirdPerson/Blueprints/BP_ThirdPersonCharacter.isDead?` (`self.Target`)))
                    (`self.SwordAttackComboCallFromBT`)
                    (set `self.mustAttack?` false)
                    (`KismetSystemLibrary.Delay` 1.0 :!label _label_4)
                    (if (> (`self.GetDistanceTo` self (`self.Target`)) 500.0)
                      _
                      (else
                        (goto _label_2)))))
                (:`OnFail`
                  (goto _label_4)))
              (else
                (switch `int` (`KismetMathLibrary.RandomIntegerInRange` 0 1) :!label _label_5
                  (:`0`
                    (goto _label_3))
                  (:`1`
                    (set `self.isStrafing?` true)
                    (switch `int` (`KismetMathLibrary.RandomIntegerInRange` 0 2)
                      (:`0`
                        (set `self.E_StrafingDirection` "NewEnumerator0"))
                      (:`1`
                        (set `self.E_StrafingDirection` "NewEnumerator2"))
                      (:`2`
                        (set `self.E_StrafingDirection` "NewEnumerator1")))
                    (`KismetSystemLibrary.Delay` 1.0)
                    (set `self.mustAttack?` true)
                    (goto _label_4))))))
          (:`OnFail`
            (goto _label_5)))
        (`self._CombatMode?` false true false 300.0)
        (if (`self.seeEnemy?`)
          (set `self.hasTarget?` false)
          (goto _label_2)
          (else
            _)))
      ;[0.05127 0.05127 0.05127] Return to post when AI can't see Player
      (`|AIMoveTo` self (`self.EnemyPost`) null 100.0
        (:`then`
          (`Widget.RemoveFromParent` (`/Game/ThirdPerson/Blueprints/BP_ThirdPersonCharacter.HUD_Widget` (stale `self.PawnSensing.OnSeePawn` _asbp_third_person_character_2))))))))

(event `ResetSense`
  ;[0.05127 0.05127 0.05127] Check if player has been seen
  (goto _label :!via `Reset`))

(fn `Attack`
  (returns (AnimationDuration :type "Float (double-precision)"))
  (`self.SwordAttackComboCallFromBT`)
  (return 0.4))

(fn `Run`
  (returns (`isRunning?` :type Boolean))
  (return false))

(fn `SetStatsByLevel`
  (`/Engine/EditorBlueprintResources/StandardMacros.Do N` (`self.Level`) :!label _label
    (:`Exit`
      (set `self.Damage` (* (`self.Damage`) 1.2))
      (set `self.XP` (* (`self.XP`) 1.2))
      (goto _label))))

(fn `SetStrafingDirection`
  (returns (StrafingDirectionVector :type "Vector Structure"))
  (bind _returnvalue (`self.GetActorRightVector`))
  (switch `/Game/DragonCore/AI_Classes/DeprecatedAI/E_StrafingDirection` (`self.E_StrafingDirection`)
    (:`NewEnumerator0`
      (set `self.StrafingDirectionVector` (* (`self.GetActorForwardVector`) -1.0)))
    (:`NewEnumerator1`
      (set `self.StrafingDirectionVector` _returnvalue))
    (:`NewEnumerator2`
      (set `self.StrafingDirectionVector` (* _returnvalue -1.0))))
  (return (`self.StrafingDirectionVector`)))

(fn `UserConstructionScript`)

(fn `Walk`
  (returns (`isWalking?` :type Boolean))
  (return false))