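; Instanced-mesh spawner component that streams idle civilian NPCs in and out around the player, using each instance as a spawn point.
; After a short delay on BeginPlay, it sizes the NPC array to the instance count and starts a slow, throttled tick.
; Each tick spawns Civilian_Idle at empty slots within SpawnRange and expires NPCs whose instance lies beyond that range plus a margin, avoiding boundary flicker.
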(event `self.ReceiveBeginPlay`
  (`self.SetComponentTickEnabled` false)
  (`self.SetComponentTickInterval` 3.0)
  (`KismetSystemLibrary.Delay` 2.0)
  (for _ (range 1 (+ (`self.GetInstanceCount`) 1))
    (`KismetArrayLibrary.Array_Add` (`self.NPC`)))
  (`self.SetComponentTickEnabled` true))

(event `self.ReceiveTick`
  (params (DeltaSeconds :type "Float (single-precision)"))
  (for (_array_element _array_index) (`self.NPC`)
    (`/Engine/EditorBlueprintResources/StandardMacros.IsValid` _array_element
      (:`Is Valid`
        (if (> (`.ReturnValue` (`self.CheckInstanceDistance` _array_index)) (+ (`self.SpawnRange`) 1000.0))
          (`Actor.SetLifeSpan` _array_element 1.0)))
      (:`Is Not Valid`
        (bind (_outinstancetransform_location _outinstancetransform_rotation _returnvalue) (`self.CheckInstanceDistance` _array_index))
        (if (< _returnvalue (`self.SpawnRange`))
          (bind _returnvalue_2 (`|SpawnActorFromClass` "/Game/DragonCore/AI_Classes/Civilians/Civilian_Idle.Civilian_Idle_C" (`KismetMathLibrary.MakeTransform` (+ _outinstancetransform_location (0.0 0.0 100.0)) _outinstancetransform_rotation) "Undefined" "OverrideRootScale" null 2 1000 1000 4 2 400 null))
          (`KismetArrayLibrary.Array_Set` (`self.NPC`) _array_index _returnvalue_2))))))