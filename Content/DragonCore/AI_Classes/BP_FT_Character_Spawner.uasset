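; BP_FT_Character_Spawner is an instanced mesh component that spawns idle civilians at its instance transforms when the player is nearby.
; After a short BeginPlay delay it builds a Civilian array with one slot per instance, then enables a throttled component tick.
; Each tick fills invalid slots within range of the player, spawning slightly above the instance, so lost civilians respawn; it never despawns them itself.
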(event `self.ReceiveBeginPlay`
  (`self.SetComponentTickEnabled` false)
  (`self.SetComponentTickInterval` 3.0)
  (`KismetSystemLibrary.Delay` 2.0)
  (for _ (range (+ (`self.GetInstanceCount`) 1))
    (`KismetArrayLibrary.Array_Add` (`self.Civilian`)))
  (`self.SetComponentTickEnabled` true))

(event `self.ReceiveTick`
  (params (DeltaSeconds :type "Float (single-precision)"))
  (for (_array_element _array_index) (`self.Civilian`)
    (`/Engine/EditorBlueprintResources/StandardMacros.IsValid` _array_element
      (:`Is Not Valid`
        (bind _outinstancetransform (`self.GetInstanceTransform` _array_index true))
        (if (< (`KismetMathLibrary.Vector_Distance` (.location _outinstancetransform) (`Actor.K2_GetActorLocation` (`GameplayStatics.GetPlayerCharacter` 0))) 5000.0)
          (bind _returnvalue (`|SpawnActorFromClass` "/Game/DragonCore/AI_Classes/Civilians/Civilian_Idle.Civilian_Idle_C" (`KismetMathLibrary.MakeTransform` (+ (.location _outinstancetransform) (0.0 0.0 100.0)) (.rotation _outinstancetransform)) "Undefined" "OverrideRootScale" null 2 1000 1000 4 2 400 null))
          (`KismetArrayLibrary.Array_Set` (`self.Civilian`) _array_index _returnvalue))))))