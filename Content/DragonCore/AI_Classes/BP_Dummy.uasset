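; BP_Dummy is a damageable dummy character that reacts to hits and ragdolls on death.
; Any damage reveals its health bar, plays a random hit montage and pitched grunt, and launches it along the player character's facing.
; BPCPlayerStats applies the damage, and its result triggers the ragdoll, sets IsDead and hides the health bar and lock-on widgets.
; Tick billboards the health bar toward the player camera.
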(event `self.ReceiveBeginPlay`
  (bind _aswb_dummy_health_bar (cast `/Game/DragonCore/UI/WB_DummyHealthBar` (`WidgetComponent.GetWidget` (`self.Health Bar Widget`))))
  (set `self.Health Bar UI` _aswb_dummy_health_bar)
  (`SceneComponent.SetVisibility` (`self.Health Bar Widget`) false false))

(event `self.ReceiveTick`
  (params (DeltaSeconds :type "Float (single-precision)"))
  (bind _health_bar_widget (`self.Health Bar Widget`))
  (`SceneComponent.K2_SetWorldRotation` _health_bar_widget (`KismetMathLibrary.FindLookAtRotation` (`SceneComponent.K2_GetComponentLocation` _health_bar_widget) (`SceneComponent.K2_GetComponentLocation` (`PlayerCameraManager.TransformComponent` (`GameplayStatics.GetPlayerCameraManager` 0)))) false false))

(event `Ragdoll`
  ;[0.05127 0.05127 0.05127] Die
  (`|ExecutionSequence`
    (:`then_0`
      (`GameplayStatics.PlaySoundAtLocation` "/Game/DragonCore/Audio/Grunts/DeathGrunt.DeathGrunt" (`self.K2_GetActorLocation`) (struct) 1.0 1.0 0.0 null null null null))
    (:`then_1`
      (`PrimitiveComponent.SetSimulatePhysics` (`self.Mesh`) true))
    (:`then_2`
      (set `self.isDead` true))))

(event `self.ReceiveAnyDamage`
  (params (Damage :type "Float (single-precision)") (DamageType :type "DamageType Object Reference") (InstigatedBy :type "Controller Object Reference") (DamageCauser :type "Actor Object Reference"))
  (`SceneComponent.SetVisibility` (`self.Health Bar Widget`) true false)
  (`self.PlayAnimMontage` (`|GetArrayItem` (`self.HitAnims`) (`KismetMathLibrary.RandomIntegerInRange` 0 (- (`KismetArrayLibrary.Array_Length` (`self.HitAnims`)) 1))))
  (bind _asbp_third_person_character (cast `/Game/ThirdPerson/Blueprints/BP_ThirdPersonCharacter` (`GameplayStatics.GetPlayerCharacter` 0)))
  (`self.LaunchCharacter` (* (`KismetMathLibrary.GetForwardVector` (`self.K2_GetActorRotation` _asbp_third_person_character)) 700))
  (`GameplayStatics.PlaySoundAtLocation` "/Game/DragonCore/Audio/Grunts/DeathGrunt.DeathGrunt" (`self.K2_GetActorLocation`) (struct) 1.0 (`KismetMathLibrary.RandomFloatInRange` 0.75 1.0) 0.0 "/Game/DragonCore/Audio/SA_Character.SA_Character" null null null)
  (bind _isplayerdead_ (`/Game/DragonCore/Blueprints/BPC_PlayerStats.Decrease Health` (`self.BPC_PlayerStats`) Damage))
  (if _isplayerdead_
    (`self.Ragdoll`)
    (`SceneComponent.SetVisibility` (`self.Health Bar Widget`) false false)
    (`SceneComponent.SetVisibility` (`self.LockOn Widget`) false false)))

(fn `UserConstructionScript`)