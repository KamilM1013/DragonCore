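; Deprecated equipment component on the third-person character that handles item pickup and toggles the gear menu.
; Interact sphere-traces from the follow camera, adds a hit item's data to the slot list and destroys the item.
; The menu input toggles the gear widget, mouse cursor and input mode, locking attacks and movement while open.
; Opening nearly freezes global time while scaling the player's time dilation to compensate; closing restores both and clears map icon widgets.
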(event `self.ReceiveBeginPlay`
  ;[0.05127 0.05127 0.05127] Event Begin Play
  (bind _asbp_third_person_character (cast `/Game/ThirdPerson/Blueprints/BP_ThirdPersonCharacter` (`self.GetOwner`)))
  (set `self.Follow Camera` (`/Game/ThirdPerson/Blueprints/BP_ThirdPersonCharacter.FollowCamera` _asbp_third_person_character))
  (set `self.BPC Attack System` (`/Game/ThirdPerson/Blueprints/BP_ThirdPersonCharacter.BPC_AttackSystem` _asbp_third_person_character))
  (set `self.Player Character` _asbp_third_person_character))

(event `EnhancedInput|/Game/ThirdPerson/Input/Actions/IA_Interact`
  (params (ActionValue :type Boolean) (ElapsedSeconds :type "Float (double-precision)") (TriggeredSeconds :type "Float (double-precision)") (InputAction :type "InputAction Object Reference" :default "/Game/ThirdPerson/Input/Actions/IA_Interact.IA_Interact"))
  (bind _follow_camera (`self.Follow Camera`))
  (bind _returnvalue (`SceneComponent.K2_GetComponentLocation` _follow_camera))
  ;[0.05127 0.05127 0.05127] PickUp Trace
  (:`Started`
    (bind (_outhit _returnvalue_2) (`KismetSystemLibrary.SphereTraceSingleForObjects` _returnvalue (+ _returnvalue (* (`KismetMathLibrary.GetForwardVector` (`SceneComponent.K2_GetComponentRotation` _follow_camera)) 1000.0)) 15.0 (`|MakeArray` "ObjectTypeQuery2" :!type "EObjectTypeQuery Enum")))
    (if _returnvalue_2
      (bind _asbp_item (cast `/Game/DragonCore/Deprecated_EquipmentSystem/BP_Item` (`.HitActor` (`GameplayStatics.BreakHitResult` _outhit))))
      (`self.AddItem` (`/Game/DragonCore/Deprecated_EquipmentSystem/BP_Item.ItemData` _asbp_item))
      (`Actor.K2_DestroyActor` _asbp_item))))

(event `EnhancedInput|/Game/ThirdPerson/Input/Actions/IA_Menu`
  (params (ActionValue :type Boolean) (ElapsedSeconds :type "Float (double-precision)") (TriggeredSeconds :type "Float (double-precision)") (InputAction :type "InputAction Object Reference" :default "/Game/ThirdPerson/Input/Actions/IA_Menu.IA_Menu"))
  (bind _returnvalue (`GameplayStatics.GetPlayerController` 0))
  (bind _bpc_attack_system (`self.BPC Attack System`))
  ;[0.05127 0.05127 0.05127] Inventory Menu Panel
  ;;[0.05127 0.05127 0.05127] Gear
  (:`Started`
    (if (not (`self.isPanelOpened?`))
      (set `/Game/DragonCore/Blueprints/BPC_AttackSystem.canDoAction?` false _bpc_attack_system)
      (bind _returnvalue_2 (`|CreateWidget` "/Game/DragonCore/Deprecated_EquipmentSystem/UI/WB_Gear.WB_Gear_C"))
      (bind _output_get (set `self.Gear Widget` _returnvalue_2))
      (`UserWidget.AddToViewport` _output_get 0)
      (set `self.isPanelOpened?` true)
      (set `PlayerController.bShowMouseCursor` true _returnvalue)
      (`WidgetBlueprintLibrary.SetInputMode_GameAndUIEx` _returnvalue (`self.Gear Widget`) "DoNotLock" false)
      (bind _asbp_third_person_character (cast `/Game/ThirdPerson/Blueprints/BP_ThirdPersonCharacter` (`self.GetOwner`)))
      (bind _charactermovement (`Character.CharacterMovement` _asbp_third_person_character))
      (`CharacterMovementComponent.SetMovementMode` _charactermovement "MOVE_None" 0)
      (`GameplayStatics.SetGlobalTimeDilation` 0.0001)
      (set `Actor.CustomTimeDilation` 10000.0 (`self.Player Character`))
      (else
        (set `/Game/DragonCore/Blueprints/BPC_AttackSystem.canDoAction?` true _bpc_attack_system)
        (bind _gear_widget (`self.Gear Widget`)
          (:`then`
            (`Widget.RemoveFromParent` _gear_widget)
            (set `self.Gear Widget` null)
            (set `self.isPanelOpened?` false)
            (set `PlayerController.bShowMouseCursor` false _returnvalue)
            (`WidgetBlueprintLibrary.SetInputMode_GameOnly` _returnvalue)
            (`CharacterMovementComponent.SetMovementMode` _charactermovement "MOVE_Walking" 0)
            (`GameplayStatics.SetGlobalTimeDilation` 1.0)
            (set `Actor.CustomTimeDilation` 1.0 (`self.Player Character`))
            (bind _foundwidgets (`WidgetBlueprintLibrary.GetAllWidgetsOfClass` "/Game/DragonCore/Deprecated_EquipmentSystem/UI/WDG_MapIcon.WDG_MapIcon_C"))
            (`Widget.RemoveFromParent` _foundwidgets))
          (:`else`))))))

(fn `AddItem`
  (params (NewItem :type "/Game/DragonCore/Deprecated_EquipmentSystem/S_Slots Structure (by ref)"))
  (`KismetArrayLibrary.Array_Add` (`self.ItemSlots`) NewItem))